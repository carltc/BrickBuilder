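; Pawn for a player-built assembly of connectable build parts, with a spring-arm camera and a toggleable physics-driven operating mode.
; Parts attach through connection slots, are tracked by GUID, respawn from data-table rows on load, and autosave on flagged modifications.
; Stored input actions route instant or continuous actions to their linked parts.
; Entering operation rebuilds changed parts into a procedural mesh with convex collision; leaving returns it to base.
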(event Custom|SaveBuildAssembly
  (params (ShouldSave :type Boolean))
  (if ShouldSave
    (Load/Save|SaveAssembly)))

(event Custom|BuildPartModifiedEvent
  (CallFunction|SaveBuildAssembly true))

(event EventBeginPlay
  (bind _proceduralmesh (Variables|Default|GetProceduralMesh))
  (bind _returnvalue (Transformation|GetWorldLocation _proceduralmesh))
  (Utilities|FlowControl|Sequence
    (:then_0
      (LocationAndRotation|SetBaseLocation _returnvalue)
      (Transformation|SetActorLocation _returnvalue false false))
    (:then_1
      (EventDispatchers|BindEventtoBuildAssemblyModified (delegate Custom|SaveBuildAssembly)))))

(fn ConstructionScript)

(fn AddBuildPart
  (params (BuildPartToAdd :type Build%20Part%20Object%20Reference) (SkipSave :type Boolean))
  (if (not (Utilities|Array|ContainsItem (Variables|Parts|GetBuildParts) BuildPartToAdd))
    (if (Utilities|Array|IsEmpty (Variables|Parts|GetBuildParts))
      (Variables|Parts|SetBaseBuildPart BuildPartToAdd)
      (Variables|/Game/Blueprints/BuildParts/BuildPart.BuildPart_C|SetIsBaseBuildPart BuildPartToAdd true))
    (Utilities|Array|Add (Variables|Parts|GetBuildParts) BuildPartToAdd)
    (Utilities|Map|Add (Variables|Data|GetBuildPartsByGuid) (Default|GetGuid BuildPartToAdd) BuildPartToAdd)
    (Transformation|AttachActorToActor BuildPartToAdd self "None" "KeepRelative" "KeepRelative" "KeepRelative" true)
    (Transformation|SetActorRelativeRotation BuildPartToAdd)
    (Default|UpdateBuildPartRelativeLocation BuildPartToAdd)
    (EventDispatchers|BindEventtoBuildPartModified BuildPartToAdd (EventDispatchers|CreateEvent :!event Custom|BuildPartModifiedEvent))
    (EventDispatchers|BindEventtoBuildAssemblyLoaded (EventDispatchers|CreateEvent BuildPartToAdd :!event ParentBuildAssemblyLoadedEvent))
    (Default|CallAddedtoBuildAssembly BuildPartToAdd)
    (Variables|Default|SetMeshNeedsRegenerating true)
    (Default|CallBuildAssemblyModified (not SkipSave))))

(fn SetBuildPartLocation
  (params (BuildPart :type Build%20Part%20Object%20Reference) (Build%20Part%20Connection%20Slot :type Build%20Part%20Connection%20Slot%20Object%20Reference) (Other%20Build%20Part%20Connection%20Slot :type Build%20Part%20Connection%20Slot%20Object%20Reference))
  (bind _parentbuildpart (Default|GetParentBuildPart Other%20Build%20Part%20Connection%20Slot))
  (bind _local_rotation (Default|GetLocalRotation _parentbuildpart))
  (Default|SetBuildAssemblyOffset BuildPart (+ (Default|GetLocalLocation _parentbuildpart) (Math|Vector|RotateVector (Variables|/Script/Engine.SceneComponent|GetRelativeLocation Other%20Build%20Part%20Connection%20Slot) _local_rotation)))
  (Default|SetCentreOffset BuildPart (Variables|/Script/Engine.SceneComponent|GetRelativeLocation Build%20Part%20Connection%20Slot) Build%20Part%20Connection%20Slot)
  (Default|SetRotation BuildPart (Math|Rotator|CombineRotators (Variables|/Script/Engine.SceneComponent|GetRelativeRotation Other%20Build%20Part%20Connection%20Slot) _local_rotation))
  (Default|SetCentreOffsetRotation BuildPart (Variables|/Script/Engine.SceneComponent|GetRelativeRotation Build%20Part%20Connection%20Slot)))

(fn GetWorldLocation
  (return (Transformation|GetWorldLocation (Variables|Default|GetSpringArm))))

(fn SetWorldLocation
  (params (NewLocation :type Vector))
  (Transformation|SetActorLocation NewLocation false false))

(fn GetBaseBuildPart
  (return (Variables|Parts|GetBaseBuildPart)))

(fn AddCameraLocalRotation
  (params (Y%20%28Pitch%29 :type Float%20%28single-precision%29) (Z%20%28Yaw%29 :type Float%20%28single-precision%29))
  (bind _springarm (Variables|Default|GetSpringArm))
  (Transformation|AddLocalRotation _springarm (Math|Rotator|MakeRotator 0.0 Y%20%28Pitch%29 0.0) false false)
  (Transformation|AddWorldRotation _springarm (Math|Rotator|MakeRotator 0.0 0.0 Z%20%28Yaw%29) false false))

(fn SetCameraZoom
  (params (Zoom%20Multiplier :type Float%20%28double-precision%29))
  (bind _springarm (Variables|Default|GetSpringArm))
  (Variables|/Script/Engine.SpringArmComponent|SetTargetArmLength _springarm (Math|Float|Clamp(Float) (* Zoom%20Multiplier (Variables|/Script/Engine.SpringArmComponent|GetTargetArmLength _springarm)) 0.0 1e+03)))

(fn GetBaseLocation
  (return (.BaseLocation (Utilities|Struct|BreakBuildAssemblyInstanceData (Variables|Data|GetBuildAssemblyInstanceData)))))

(fn SetBaseLocation
  (params (BaseLocation :type Vector))
  (Utilities|Struct|SetmembersinBuildAssemblyInstanceData (Variables|Data|GetBuildAssemblyInstanceData) BaseLocation))

(fn ResetCamera
  (Variables|/Script/Engine.SpringArmComponent|SetTargetArmLength (Variables|Default|GetSpringArm) 3e+02)
  (Camera|SetCameraRotation 3e+01 0.0))

(fn SetCameraRotation
  (params (Y%20%28Pitch%29 :type Float%20%28single-precision%29) (Z%20%28Yaw%29 :type Float%20%28single-precision%29))
  (bind _springarm (Variables|Default|GetSpringArm))
  (Transformation|SetWorldRotation _springarm (Math|Rotator|MakeRotator 0.0 0.0 Z%20%28Yaw%29) false false)
  (Transformation|SetRelativeRotation _springarm (Math|Rotator|MakeRotator 0.0 Y%20%28Pitch%29 0.0) false false))

(fn PerformInputInstantAction
  (params (Input%20Type :type InputType%20Enum :default "NewEnumerator0"))
  (bind _inputactions1 (Properties|GetInputActions))
  (bind _keys (Utilities|Map|Keys _inputactions1))
  (for _array_element _keys
    (if (Utilities|Enum|Equal(Enum) (.InputType (Utilities|Struct|BreakInputAction (.Value (Utilities|Map|Find _inputactions1 _array_element)))) Input%20Type)
      (bind _result (Utilities|Set|ToArray (.BuildPartGuids (Utilities|Struct|BreakInputAction (.Value (Utilities|Map|Find _inputactions1 _array_element))))))
      (for _array_element_2 _result
        (bind _build_part (Utilities|GetBuildPart _array_element_2)
          (:Found
            (Default|PerformInstantActions _build_part (.InputValue (Utilities|Struct|BreakInputAction (.Value (Utilities|Map|Find _inputactions1 _array_element)))))))))))

(fn SetInputContinuousActionsRunning
  (params (Input%20Type :type InputType%20Enum :default "NewEnumerator0") (Should%20Run :type Boolean))
  (bind _inputactions1 (Properties|GetInputActions))
  (bind _keys (Utilities|Map|Keys _inputactions1))
  (for _array_element _keys
    (if (Utilities|Enum|Equal(Enum) (.InputType (Utilities|Struct|BreakInputAction (.Value (Utilities|Map|Find _inputactions1 _array_element)))) Input%20Type)
      (bind _result (Utilities|Set|ToArray (.BuildPartGuids (Utilities|Struct|BreakInputAction (.Value (Utilities|Map|Find _inputactions1 _array_element))))))
      (for _array_element_2 _result
        (bind _build_part (Utilities|GetBuildPart _array_element_2)
          (:Found
            (Default|SetContinuousActionsRunning _build_part Should%20Run (.InputValue (Utilities|Struct|BreakInputAction (.Value (Utilities|Map|Find _inputactions1 _array_element)))))))))))

(fn SaveAssembly
  (bind _returnvalue (SaveGame|CreateSaveGameObject "/Game/Blueprints/Saving/BuildAssemblySave.BuildAssemblySave_C"))
  (LocalVariables|SetNewAssemblySave _returnvalue)
  (Utilities|FlowControl|Sequence
    (:then_0
      (Variables|/Game/Blueprints/Saving/BuildAssemblySave.BuildAssemblySave_C|SetBuildAssemblyInstanceData (LocalVariables|GetNewAssemblySave) (Variables|Data|GetBuildAssemblyInstanceData)))
    (:then_1
      (for _array_element (Variables|Parts|GetBuildParts)
        (Utilities|Array|Add (Variables|/Game/Blueprints/Saving/BuildAssemblySave.BuildAssemblySave_C|GetBuildPartsInstanceData (LocalVariables|GetNewAssemblySave)) (Default|GetBuildPartInstanceData _array_element))))
    (:then_2
      (bind _returnvalue_2 (SaveGame|SaveGametoSlot (LocalVariables|GetNewAssemblySave) (Properties|GetBuildAssemblySaveName)))
      (if _returnvalue_2
        (Development|PrintString "Save successful!" true false "(R=0.000000,G=1.000000,B=0.010000,A=1.000000)" 1e+01)))))

(fn GetGuid
  (if (not (== (.Guid (Utilities|Struct|BreakBuildPartInstanceData (Utilities|Struct|MakeBuildPartInstanceData "00000000000000000000000000000000" "None"))) (.BuildAssemblyGuid (Utilities|Struct|BreakBuildAssemblyInstanceData (Variables|Data|GetBuildAssemblyInstanceData)))))
    _
    (else
      (Utilities|Struct|SetmembersinBuildAssemblyInstanceData (Variables|Data|GetBuildAssemblyInstanceData) (Guid|NewGuid))))
  (return (.BuildAssemblyGuid (Utilities|Struct|BreakBuildAssemblyInstanceData (Variables|Data|GetBuildAssemblyInstanceData)))))

(fn LoadBuildParts
  (params (BuildPartsInstanceData :type Array%20of%20Build%20Part%20Instance%20Data%20Structures))
  (for _array_element BuildPartsInstanceData
    (bind _returnvalue (Utilities|GetDataTableRow "/Game/Blueprints/BuildParts/BuildParts/BuildParts.BuildParts" (.BuildPartRowName (Utilities|Struct|BreakBuildPartInstanceData _array_element)))
      (:then
        (bind _returnvalue_2 (Game|SpawnActorfromClass (.Class (Utilities|Struct|BreakBuildPartData _returnvalue)) (Math|Transform|MakeTransform "0, 0, 0") "Undefined" "MultiplyWithRoot" 0 _array_element true 0))
        (BuildParts|AddBuildPart _returnvalue_2 true)
        (Default|ConnectUnconnectedSlots _returnvalue_2))))
  (Default|CallBuildAssemblyLoaded))

(fn GetBuildPartbyGuid
  (params (Key :type Guid%20Structure%20%28by%20ref%29))
  (bind _buildpartsbyguid (Variables|Data|GetBuildPartsByGuid))
  (bind (_value _returnvalue) (Utilities|Map|Find _buildpartsbyguid Key))
  (return _value _returnvalue))

(fn GetBuildAssemblySaveName
  (if (not (Utilities|Array|IsEmpty (.BuildAssemblySaveName (Utilities|Struct|BreakBuildAssemblyInstanceData (Variables|Data|GetBuildAssemblyInstanceData)))))
    _
    (else
      (Utilities|Struct|SetmembersinBuildAssemblyInstanceData (Variables|Data|GetBuildAssemblyInstanceData) (Utilities|String|Append "BuildAssembly-" (Guid|ToString(Guid) (Properties|GetGuid))))))
  (return (.BuildAssemblySaveName (Utilities|Struct|BreakBuildAssemblyInstanceData (Variables|Data|GetBuildAssemblyInstanceData)))))

(fn RegenerateAssemblyMesh
  (if (Variables|Default|GetMeshNeedsRegenerating)
    (Class|ProceduralMeshComponent|ClearAllMeshSections (Variables|Default|GetProceduralMesh))
    (for (_array_element _array_index) (Variables|Parts|GetBuildParts)
      (bind (_vertices _triangles _normals _uvs) (Class|KismetProceduralMeshLibrary|GetSectionfromStaticMesh (Variables|/Script/Engine.StaticMeshComponent|GetStaticMesh (Variables|/Game/Blueprints/BuildParts/BuildPart.BuildPart_C|GetStaticMesh _array_element)) 3))
      (bind _rotated_vertices (ProceduralMesh|RotateandMoveVertices _vertices (Default|GetLocalRotation _array_element) (Default|GetLocalLocation _array_element)))
      (bind (_normals_2 _tangents) (Class|KismetProceduralMeshLibrary|CalculateTangentsforMesh _rotated_vertices _triangles _uvs))
      (Class|ProceduralMeshComponent|CreateMeshSectionLinearColor (Variables|Default|GetProceduralMesh) _array_index _rotated_vertices _triangles _normals_2 _uvs 0 0 0 0 _tangents false false)
      (Class|ProceduralMeshComponent|AddCollisionConvexMesh (Variables|Default|GetProceduralMesh) _rotated_vertices))
    (Variables|Default|SetMeshNeedsRegenerating false)))

(fn RotateandMoveVertices
  (params (Vertices :type Array%20of%20Vectors) (Rotation :type Rotator) (Location :type Vector))
  (for _array_element Vertices
    (Utilities|Array|Add (LocalVariables|GetNew%20Rotated%20Vertices) (+ (Math|Vector|RotateVector _array_element Rotation) Location)))
  (return (LocalVariables|GetNew%20Rotated%20Vertices)))

(fn GetBuildPartSlotLocationandRotation
  (params (BuildPart :type Build%20Part%20Object%20Reference) (Slot%20Relative%20Location :type Vector) (Slot%20Relative%20Rotation :type Rotator))
  (bind _local_rotation (Default|GetLocalRotation BuildPart))
  (return (+ (Default|GetLocalLocation BuildPart) (Math|Vector|RotateVector Slot%20Relative%20Location _local_rotation)) (Math|Rotator|CombineRotators Slot%20Relative%20Rotation _local_rotation)))

(fn GetInputActions
  (return (.InputActions (Utilities|Struct|BreakBuildAssemblyInstanceData (Variables|Data|GetBuildAssemblyInstanceData)))))

(fn SetInputActionProperties
  (params (New%20Input%20Action%20Values :type Input%20Action%20Structure%20%28by%20ref%29))
  (bind _output_get (LocalVariables|SetInputActions (.InputActions (Utilities|Struct|BreakBuildAssemblyInstanceData (Variables|Data|GetBuildAssemblyInstanceData)))))
  (Utilities|Map|Add _output_get (.Guid (Utilities|Struct|BreakInputAction New%20Input%20Action%20Values)) New%20Input%20Action%20Values)
  (Utilities|Struct|SetmembersinBuildAssemblyInstanceData (Variables|Data|GetBuildAssemblyInstanceData) (LocalVariables|GetInputActions))
  (Default|CallBuildAssemblyModified true))

(fn AddInputAction
  (params (InputType :type InputType%20Enum :default "NewEnumerator0") (BuildPartGuids1 :type Set%20of%20Guid%20Structures))
  (bind _output_get (LocalVariables|SetNewGuid (Guid|NewGuid)))
  (Actions|SetInputActionProperties (Utilities|Struct|MakeInputAction _output_get InputType BuildPartGuids1))
  (return (.Input%20Action (Properties|GetInputAction (LocalVariables|GetNewGuid)))))

(fn ToggleBuildPartinInputAction
  (params (InputActionGuid :type Guid%20Structure%20%28by%20ref%29) (BuildPartGuid :type Guid%20Structure))
  (bind _output_get (LocalVariables|SetInputActions (.InputActions (Utilities|Struct|BreakBuildAssemblyInstanceData (Variables|Data|GetBuildAssemblyInstanceData)))))
  (if (.ReturnValue (Utilities|Map|Find _output_get InputActionGuid))
    (bind _output_get_2 (LocalVariables|SetSelectedInputAction (.Value (Utilities|Map|Find _output_get InputActionGuid))))
    (if (Utilities|Set|Contains (.BuildPartGuids (Utilities|Struct|BreakInputAction _output_get_2)) BuildPartGuid)
      (Utilities|Set|Remove (.BuildPartGuids (Utilities|Struct|BreakInputAction _output_get_2)) BuildPartGuid)
      (else
        (Utilities|Set|Add (.BuildPartGuids (Utilities|Struct|BreakInputAction _output_get_2)) BuildPartGuid)))
    (Utilities|Map|Add (LocalVariables|GetInputActions) InputActionGuid (LocalVariables|GetSelectedInputAction))
    (Utilities|Struct|SetmembersinBuildAssemblyInstanceData (Variables|Data|GetBuildAssemblyInstanceData) (LocalVariables|GetInputActions))
    (Default|CallBuildAssemblyModified true)))

(fn GetInputAction
  (params (Guid :type Guid%20Structure%20%28by%20ref%29))
  (bind _buildassemblyinstancedata (Variables|Data|GetBuildAssemblyInstanceData))
  (bind _inputactions (Utilities|Struct|BreakBuildAssemblyInstanceData _buildassemblyinstancedata))
  (bind (_value _returnvalue) (Utilities|Map|Find _inputactions Guid))
  (return _value _returnvalue))

(fn RemoveBuildPart
  (params (BuildPartToRemove :type Build%20Part%20Object%20Reference))
  (if (Utilities|Array|ContainsItem (Variables|Parts|GetBuildParts) BuildPartToRemove)
    (if (== (Variables|Parts|GetBaseBuildPart) BuildPartToRemove)
      (return false)
      (else
        (Utilities|Array|RemoveItem (Variables|Parts|GetBuildParts) BuildPartToRemove)
        (Utilities|Map|Remove (Variables|Data|GetBuildPartsByGuid) (Default|GetGuid BuildPartToRemove))
        (EventDispatchers|UnbindallEventsfromBuildPartModified BuildPartToRemove)
        (EventDispatchers|UnbindEventfromBuildAssemblyLoaded (EventDispatchers|CreateEvent BuildPartToRemove :!event ParentBuildAssemblyLoadedEvent))
        (for _array_element (Default|GetChildBuildParts BuildPartToRemove)
          (BuildParts|RemoveBuildPart _array_element))
        (Default|DisconnectNonChildSlots BuildPartToRemove)
        (Variables|Default|SetMeshNeedsRegenerating true)
        (Default|CallBuildAssemblyModified false)
        (return true)))
    (else
      (return true))))

(fn GetBuildAssemblyOperating
  (return (Variables|Operating|GetBuildAssemblyOperating)))

(fn SetBuildAssemblyOperating
  (params (BuildAssemblyOperating :type Boolean))
  (bind _output_get (Variables|Operating|SetBuildAssemblyOperating BuildAssemblyOperating))
  (if _output_get
    (ProceduralMesh|RegenerateAssemblyMesh)
    (else
      (Transformation|SetActorLocation (LocationAndRotation|GetBaseLocation) false false)
      (Transformation|SetActorRotation (Math|Rotator|MakeRotator 0.0 0.0 0.0))))
  (Physics|SetSimulatePhysics (Variables|Default|GetProceduralMesh) (Variables|Operating|GetBuildAssemblyOperating))
  (Camera|SetCameraRotation -3e+01 0.0))

(fn PerformInputActions
  (params (Input%20Type :type InputType%20Enum :default "NewEnumerator0") (Should%20Run :type Boolean))
  (bind _inputactions1 (Properties|GetInputActions))
  (bind _keys (Utilities|Map|Keys _inputactions1))
  (for _array_element _keys
    (if (Utilities|Enum|Equal(Enum) (.InputType (Utilities|Struct|BreakInputAction (.Value (Utilities|Map|Find _inputactions1 _array_element)))) Input%20Type)
      (bind _result (Utilities|Set|ToArray (.BuildPartGuids (Utilities|Struct|BreakInputAction (.Value (Utilities|Map|Find _inputactions1 _array_element))))))
      (for _array_element_2 _result
        (bind _build_part (Utilities|GetBuildPart _array_element_2)
          (:Found
            (if (.Continuous (Utilities|Struct|BreakInputAction (.Value (Utilities|Map|Find _inputactions1 _array_element))))
              (Default|SetContinuousActionsRunning _build_part Should%20Run (.InputValue (Utilities|Struct|BreakInputAction (.Value (Utilities|Map|Find _inputactions1 _array_element)))) (.Guid (Utilities|Struct|BreakInputAction (.Value (Utilities|Map|Find _inputactions1 _array_element)))))
              (elif Should%20Run
                (Default|PerformInstantActions _build_part (.InputValue (Utilities|Struct|BreakInputAction (.Value (Utilities|Map|Find _inputactions1 _array_element)))))))))))))

(fn GetNearestConnectionSlot
  (params (Mouse%20Location :type Vector) (ActorsToIgnore :type Array%20of%20Actor%20Object%20References))
  (bind (_outhits _returnvalue) (Class|KismetSystemLibrary|BoxTraceMulti Mouse%20Location Mouse%20Location "3.000000,3.000000,0.500000" "0, 0, 0" "TraceTypeQuery3" false ActorsToIgnore "ForOneFrame" true "(R=1.000000,G=0.000000,B=0.000000,A=1.000000)" "(R=0.000000,G=1.000000,B=0.000000,A=1.000000)" 0.0))
  (if _returnvalue
    (for _array_element _outhits
      (bind _asbuild_part_connection_slot (Utilities|Casting|CastToBuildPartConnectionSlot (.HitComponent (Collision|BreakHitResult _array_element))))
      (if (not (Default|IsConnected _asbuild_part_connection_slot))
        (Utilities|IsValid (LocalVariables|GetClosestConnectionSlot)
          (:Is%20Valid
            (if (< (Math|Vector|Distance(Vector) (Transformation|GetWorldLocation _asbuild_part_connection_slot) Mouse%20Location) (LocalVariables|GetMinDistance))
              (LocalVariables|SetClosestConnectionSlot _asbuild_part_connection_slot :!label _label)
              (LocalVariables|SetMinDistance (Math|Vector|Distance(Vector) (Transformation|GetWorldLocation _asbuild_part_connection_slot) Mouse%20Location))))
          (:Is%20Not%20Valid
            (goto _label)))))
    (return (LocalVariables|GetClosestConnectionSlot) (Utilities|IsValid (LocalVariables|GetClosestConnectionSlot)))))

(fn RecalculateBuildPartDescendants
  (Default|RecalculateDescendantBuildParts (BuildParts|GetBaseBuildPart)))