(event EventBeginPlay
  (CallFunction|AddBuildPart (CallFunction|GetBaseBuildPart)))

(event Collision|EventActorBeginOverlap
  (params (OtherActor :type Actor%20Object%20Reference)))

(event EventTick
  (params (DeltaSeconds :type Float%20%28single-precision%29)))

(fn ConstructionScript)

(fn AddBuildPart
  (params (BuildPartToAdd :type Build%20Part%20Object%20Reference))
  (if (not (Utilities|Array|ContainsItem (Variables|Parts|GetBuildParts) BuildPartToAdd))
    (Utilities|Array|Add (Variables|Parts|GetBuildParts) BuildPartToAdd)
    (Transformation|AttachActorToActor BuildPartToAdd self "None" "KeepRelative" "KeepRelative" "KeepRelative" true)
    (Transformation|SetActorRelativeRotation BuildPartToAdd)))

(fn GetNearestUnconnectedSlot
  (params (Socket%20Type :type BuildPartSocketType%20Enum :default "NewEnumerator0") (Location :type Vector) (BuildPartToAvoid :type Build%20Part%20Object%20Reference))
  (for _array_element (Variables|Parts|GetBuildParts)
    (if (not (== _array_element BuildPartToAvoid))
      (for _array_element_2 (Default|GetUnconnectedSlots _array_element Socket%20Type)
        (Utilities|IsValid (LocalVariables|GetCurrentNearestConnectionSlot)
          (:Is%20Valid
            (if (< (Math|Vector|Distance(Vector) (Transformation|GetWorldLocation _array_element_2) Location) (LocalVariables|GetCurrentSmallestDistance))
              (LocalVariables|SetCurrentNearestConnectionSlot _array_element_2 :!label _label)
              (LocalVariables|SetCurrentSmallestDistance (Math|Vector|Distance(Vector) (Transformation|GetWorldLocation _array_element_2) Location))))
          (:Is%20Not%20Valid
            (goto _label))))))
  (return (LocalVariables|GetCurrentNearestConnectionSlot) (Utilities|IsValid (LocalVariables|GetCurrentNearestConnectionSlot))))

(fn AddStartingBuildPart
  (bind _returnvalue (Game|SpawnActorfromClass "/Game/Blueprints/BuildParts/BuildParts/Bricks/BP_Brick_2x2.BP_Brick_2x2_C" (Math|Transform|MakeTransform "0, 0, 0") "Undefined" "MultiplyWithRoot" 0 false 0))
  (Transformation|AttachActorToActor _returnvalue self "None" "KeepRelative" "KeepRelative" "KeepRelative" true)
  (Utilities|Array|Add (Variables|Parts|GetBuildParts) _returnvalue))

(fn SetBuildPartLocation
  (params (BuildPart :type Build%20Part%20Object%20Reference) (Build%20Part%20Connection%20Slot :type Build%20Part%20Connection%20Slot%20Object%20Reference) (Other%20Build%20Part%20Connection%20Slot :type Build%20Part%20Connection%20Slot%20Object%20Reference))
  (bind _parentbuildpart (Default|GetParentBuildPart Other%20Build%20Part%20Connection%20Slot))
  (bind _relativerotation (Variables|/Script/Engine.SceneComponent|GetRelativeRotation Other%20Build%20Part%20Connection%20Slot))
  (bind _relativerotation_2 (Variables|/Script/Engine.SceneComponent|GetRelativeRotation Build%20Part%20Connection%20Slot))
  (bind _local_rotation (Default|GetLocalRotation _parentbuildpart))
  (bind _returnvalue (Math|Rotator|CombineRotators _relativerotation _local_rotation))
  (Default|SetBuildAssemblyOffset BuildPart (+ (Default|GetRelativeLocation _parentbuildpart) (Math|Vector|RotateVector (Variables|/Script/Engine.SceneComponent|GetRelativeLocation Other%20Build%20Part%20Connection%20Slot) _local_rotation)))
  (Default|SetCentreOffset BuildPart (Variables|/Script/Engine.SceneComponent|GetRelativeLocation Build%20Part%20Connection%20Slot))
  (Default|SetRotation BuildPart _returnvalue)
  (Default|SetCentreOffsetRotation BuildPart _relativerotation_2)
  (Development|PrintString (Utilities|String|Append "Old Slot:" (Utilities|String|ToString(Rotator) _relativerotation)) true false "(R=0.000000,G=0.660000,B=1.000000,A=1.000000)" 0.0)
  (Development|PrintString (Utilities|String|Append "Old Part:" (Utilities|String|ToString(Rotator) _local_rotation)) true false "(R=0.000000,G=0.660000,B=1.000000,A=1.000000)" 0.0)
  (Development|PrintString (Utilities|String|Append "New Slot:" (Utilities|String|ToString(Rotator) _relativerotation_2)) true false "(R=0.000000,G=0.660000,B=1.000000,A=1.000000)" 0.0)
  (Development|PrintString (Utilities|String|Append "New Part:" (Utilities|String|ToString(Rotator) _returnvalue)) true false "(R=0.000000,G=0.660000,B=1.000000,A=1.000000)" 0.0))

(fn GetWorldLocation
  (return (Transformation|GetWorldLocation (Variables|Default|GetChildActor))))

(fn SetWorldLocation
  (params (NewLocation :type Vector))
  (Transformation|SetActorLocation NewLocation false false))

(fn BeginPlayMode
  (Utilities|FlowControl|Sequence
    (:then_0
      (for _array_element (Variables|Parts|GetBuildParts)
        (Default|SetSimulatePhysics _array_element true)))
    (:then_1
      (CallFunction|SpawnPhysicsConstraints))))

(fn BeginBuildMode
  (Utilities|FlowControl|Sequence
    (:then_0
      (CallFunction|ClearPhysicsContraints))
    (:then_1
      (for _array_element (Variables|Parts|GetBuildParts)
        (Default|SetSimulatePhysics _array_element false)
        (if (== _array_element (CallFunction|GetBaseBuildPart))
          (Transformation|AttachComponentToComponent _array_element (Variables|Default|GetChildActor) "None" "KeepRelative" "KeepRelative" "KeepRelative" false)
          (else
            (Transformation|AttachActorToActor _array_element self "None" "KeepRelative" "KeepRelative" "KeepRelative" false)))
        (Default|UpdateBuildPartRelativeLocation _array_element)))))

(fn GetBaseBuildPart
  (Utilities|IsValid (Variables|Default|GetBaseBuildPart)
    (:Is%20Valid
      _)
    (:Is%20Not%20Valid
      (bind _asbuild_part (Utilities|Casting|CastToBuildPart (Variables|/Script/Engine.ChildActorComponent|GetChildActor (Variables|Default|GetChildActor)))
        (:then
          (Variables|Default|SetBaseBuildPart _asbuild_part))
        (:CastFailed
          _))))
  (return (Variables|Default|GetBaseBuildPart)))

(fn SpawnPhysicsConstraints
  (for _array_element (Variables|Parts|GetBuildParts)
    (if (not (== _array_element (CallFunction|GetBaseBuildPart)))
      (bind _returnvalue (Game|SpawnActorfromClass "/Script/Engine.PhysicsConstraintActor" (Math|Transform|MakeTransform "0, 0, 0") "Undefined" "MultiplyWithRoot" 0 0))
      (Utilities|Array|Add (Variables|Default|GetPhysicsConstraints) _returnvalue)
      (Class|PhysicsConstraintComponent|SetConstrainedComponents (Variables|/Script/Engine.PhysicsConstraintActor|GetConstraintComp _returnvalue) (Variables|/Game/Blueprints/BuildParts/BuildPart.BuildPart_C|GetStaticMesh (CallFunction|GetBaseBuildPart)) "None" (Variables|/Game/Blueprints/BuildParts/BuildPart.BuildPart_C|GetStaticMesh _array_element) "None")
      (Utilities|FlowControl|Sequence
        (:then_0
          (Class|PhysicsConstraintComponent|SetLinearXLimit (Variables|/Script/Engine.PhysicsConstraintActor|GetConstraintComp _returnvalue) "LCM_Locked" 0.0)
          (Class|PhysicsConstraintComponent|SetAngularSwing1Limit (Variables|/Script/Engine.PhysicsConstraintActor|GetConstraintComp _returnvalue) "ACM_Locked" 0.0))
        (:then_1
          (Class|PhysicsConstraintComponent|SetLinearYLimit (Variables|/Script/Engine.PhysicsConstraintActor|GetConstraintComp _returnvalue) "LCM_Locked" 0.0)
          (Class|PhysicsConstraintComponent|SetAngularSwing2Limit (Variables|/Script/Engine.PhysicsConstraintActor|GetConstraintComp _returnvalue) "ACM_Locked" 0.0))
        (:then_2
          (Class|PhysicsConstraintComponent|SetLinearZLimit (Variables|/Script/Engine.PhysicsConstraintActor|GetConstraintComp _returnvalue) "LCM_Locked" 0.0)
          (Class|PhysicsConstraintComponent|SetAngularTwistLimit (Variables|/Script/Engine.PhysicsConstraintActor|GetConstraintComp _returnvalue) "ACM_Locked" 0.0))))))

(fn ClearPhysicsContraints
  (bind _physicsconstraints (Variables|Default|GetPhysicsConstraints))
  (for _array_element _physicsconstraints
    (Actor|DestroyActor _array_element))
  (Utilities|Array|Clear _physicsconstraints))

(fn GetBaseLocation
  (return (Utilities|Struct|BreakBuildAssemblyInstanceData (Variables|Default|GetBuildAssemblyInstanceData))))

(fn SetBaseLocation
  (params (BaseLocation :type Vector))
  (Utilities|Struct|SetmembersinBuildAssemblyInstanceData (Variables|Default|GetBuildAssemblyInstanceData) BaseLocation))