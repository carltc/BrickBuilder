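; Actor for a single modular part in a player-built assembly pawn, holding its instance data, connection slots and actions.
; It caches male and female unconnected slots, links them when added to an assembly, and picks non-overlapping slots by seed for attachment.
; Offset, 90-degree step and rotation setters recompute the relative transform from instance data.
; Instant and continuous action components are gathered and triggered through the part.
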(event Custom|ParentBuildAssemblyLoadedEvent
  (Default|CallParentBuildAssemblyLoaded (Data|GetParentBuildAssembly)))

(event Custom|SubscribeToConnectionSlotsConnectedEvent
  (for _array_element (Actor|GetComponentsByClass "/Game/Blueprints/BuildParts/BuildPartConnectionSlot.BuildPartConnectionSlot_C")
    (EventDispatchers|BindEventtoConnected _array_element (delegate Custom|ConnectionSlotConnectedEvent))))

(event Custom|ConnectionSlotConnectedEvent
  (params (Connected%20Slot :type Build%20Part%20Connection%20Slot%20Object%20Reference))
  (bind _returnvalue (Utilities|Array|RemoveItem (Variables|ConnectionSlots|GetFemaleUnconnectedSlots) Connected%20Slot))
  (if _returnvalue
    _
    (else
      (Utilities|Array|RemoveItem (Variables|ConnectionSlots|GetMaleUnconnectedSlots) Connected%20Slot)))
  (Default|CallConnectionSlotConnected Connected%20Slot))

(event Custom|AddedToBuildAssemblyEvent
  (CallFunction|ConnectSlots))

(event EventBeginPlay
  (Utilities|FlowControl|Sequence
    (:then_0
      (ConnectionSlots|RecalculateConnectionSlots))
    (:then_1
      (Actions|RecalculateActions))
    (:then_2
      (bind _returnvalue (Utilities|GetDataTableRow "/Game/Blueprints/BuildParts/BuildParts/BuildParts.BuildParts" (.BuildPartRowName (Utilities|Struct|BreakBuildPartInstanceData (Variables|Data|GetBuildPartInstanceData))))
        (:then
          (Variables|Data|SetBuildPartData _returnvalue))))
    (:then_3
      (CallFunction|SubscribetoConnectionSlotsConnectedEvent))
    (:then_4
      (EventDispatchers|BindEventtoAddedtoBuildAssembly (delegate Custom|AddedToBuildAssemblyEvent)))))

(fn ConstructionScript)

(fn GetValidConnectionSlot
  (params (SocketSeed :type Integer) (Connecting%20To :type Build%20Part%20Connection%20Slot%20Object%20Reference))
  (bind _unconnectedconnectionslots (LocalVariables|GetUnconnectedConnectionSlots))
  (switch Utilities|FlowControl|Switch|SwitchonBuildPartConnectionSlotType (Variables|/Game/Blueprints/BuildParts/BuildPartConnectionSlot.BuildPartConnectionSlot_C|GetConnectionSlotType Connecting%20To)
    (:NewEnumerator0
      (LocalVariables|SetConnectionSlotsToCheck (Variables|ConnectionSlots|GetFemaleUnconnectedSlots)))
    (:NewEnumerator1
      (LocalVariables|SetConnectionSlotsToCheck (Variables|ConnectionSlots|GetMaleUnconnectedSlots)))
    (:NewEnumerator2
      (Development|PrintString (Utilities|String|MakeLiteralString "Could not get a valid Connection Slot of type 'Either'"))
      (return false 0)))
  (for _array_element (LocalVariables|GetConnectionSlotsToCheck)
    (if (Default|IsConnected _array_element)
      (Development|PrintString "Hello")
      (else
        (LocationAndRotation|SetCentreOffset self (Variables|/Script/Engine.SceneComponent|GetRelativeLocation _array_element))
        (if (Overlaps|OverlapsOtherBuildParts self)
          (Development|PrintString "Hello")
          (else
            (Utilities|Array|Add (LocalVariables|GetUnconnectedConnectionSlots) _array_element))))))
  (return (Utilities|Array|IsNotEmpty _unconnectedconnectionslots) (Utilities|Array|Get(acopy) _unconnectedconnectionslots (Math|Integer|%(Integer) SocketSeed (Utilities|Array|Length _unconnectedconnectionslots)))))

(fn RecalculateConnectionSlots
  (Utilities|Array|Clear (Variables|ConnectionSlots|GetMaleUnconnectedSlots))
  (Utilities|Array|Clear (Variables|ConnectionSlots|GetFemaleUnconnectedSlots))
  (for _array_element (Actor|GetComponentsByClass "/Game/Blueprints/BuildParts/BuildPartConnectionSlot.BuildPartConnectionSlot_C")
    (if (not (Default|IsConnected _array_element))
      (switch Utilities|FlowControl|Switch|SwitchonBuildPartConnectionSlotType (Variables|/Game/Blueprints/BuildParts/BuildPartConnectionSlot.BuildPartConnectionSlot_C|GetConnectionSlotType _array_element)
        (:NewEnumerator0
          (Utilities|Array|Add (Variables|ConnectionSlots|GetMaleUnconnectedSlots) _array_element))
        (:NewEnumerator1
          (Utilities|Array|Add (Variables|ConnectionSlots|GetFemaleUnconnectedSlots) _array_element))))))

(fn GetUnconnectedSlots
  (params (Slot%20Type :type BuildPartConnectionSlotType%20Enum :default "NewEnumerator0"))
  (switch Utilities|FlowControl|Switch|SwitchonBuildPartConnectionSlotType Slot%20Type
    (:NewEnumerator0
      (return (Variables|ConnectionSlots|GetMaleUnconnectedSlots)))
    (:NewEnumerator1
      (return (Variables|ConnectionSlots|GetFemaleUnconnectedSlots)))
    (:NewEnumerator2
      (Utilities|Array|AppendArray (LocalVariables|GetAllUnconnectedSlots) (Variables|ConnectionSlots|GetFemaleUnconnectedSlots))
      (Utilities|Array|AppendArray (LocalVariables|GetAllUnconnectedSlots) (Variables|ConnectionSlots|GetMaleUnconnectedSlots))
      (return (LocalVariables|GetAllUnconnectedSlots)))))

(fn GetWorldLocation
  (return (Transformation|GetWorldLocation (Variables|Default|GetStaticMesh))))

(fn OverlapsOtherBuildParts
  (return (Utilities|Array|IsNotEmpty (Collision|GetOverlappingActors (Variables|Default|GetStaticMesh) "BuildPart_C" :!class /Script/Engine.PrimitiveComponent))))

(fn GetLocalLocation
  (return (- (LocationAndRotation|GetBuildAssemblyOffset) (Math|Vector|RotateVector (LocationAndRotation|GetCentreOffset) (LocationAndRotation|GetLocalRotation)))))

(fn SetRelative90
  (params (Rotation90 :type Integer))
  (Utilities|Struct|SetmembersinBuildPartInstanceData (Variables|Data|GetBuildPartInstanceData) Rotation90)
  (LocationAndRotation|UpdateBuildPartRelativeLocation))

(fn IncrementRotation90
  (LocationAndRotation|SetRelative90 (Math|Integer|%(Integer) (+ (.Rotation90 (Utilities|Struct|BreakBuildPartInstanceData (Variables|Data|GetBuildPartInstanceData))) 1) 4)))

(fn SetCentreOffset
  (params (CentreOffset :type Vector))
  (Utilities|Struct|SetmembersinBuildPartInstanceData (Variables|Data|GetBuildPartInstanceData) CentreOffset)
  (LocationAndRotation|UpdateBuildPartRelativeLocation))

(fn GetCentreOffset
  (return (.CentreOffset (Utilities|Struct|BreakBuildPartInstanceData (Variables|Data|GetBuildPartInstanceData)))))

(fn SetBuildAssemblyOffset
  (params (BuildAssemblyOffset :type Vector))
  (Utilities|Struct|SetmembersinBuildPartInstanceData (Variables|Data|GetBuildPartInstanceData) BuildAssemblyOffset)
  (LocationAndRotation|UpdateBuildPartRelativeLocation))

(fn GetBuildAssemblyOffset
  (return (.BuildAssemblyOffset (Utilities|Struct|BreakBuildPartInstanceData (Variables|Data|GetBuildPartInstanceData)))))

(fn UpdateBuildPartRelativeLocation
  (Transformation|SetActorRelativeLocation (LocationAndRotation|GetLocalLocation))
  (Transformation|SetActorRelativeRotation (LocationAndRotation|GetLocalRotation)))

(fn GetRotation90
  (return (.Rotation90 (Utilities|Struct|BreakBuildPartInstanceData (Variables|Data|GetBuildPartInstanceData)))))

(fn GetRotation
  (return (.Rotation (Utilities|Struct|BreakBuildPartInstanceData (Variables|Data|GetBuildPartInstanceData)))))

(fn SetRotation
  (params (Rotation1 :type Rotator))
  (Utilities|Struct|SetmembersinBuildPartInstanceData (Variables|Data|GetBuildPartInstanceData) Rotation1)
  (LocationAndRotation|UpdateBuildPartRelativeLocation))

(fn GetCentreOffsetRotation
  (return (.CentreOffsetRotation (Utilities|Struct|BreakBuildPartInstanceData (Variables|Data|GetBuildPartInstanceData)))))

(fn SetCentreOffsetRotation
  (params (CentreOffsetRotation :type Rotator))
  (Utilities|Struct|SetmembersinBuildPartInstanceData (Variables|Data|GetBuildPartInstanceData) CentreOffsetRotation)
  (LocationAndRotation|UpdateBuildPartRelativeLocation))

(fn GetLocalRotation
  (return (Math|Rotator|CombineRotators (Math|Rotator|CombineRotators (Class|KismetMathLibrary|NegateRotator (LocationAndRotation|GetCentreOffsetRotation)) (Math|Rotator|MakeRotator 0.0 0.0 (* (LocationAndRotation|GetRotation90) 9e+01))) (LocationAndRotation|GetRotation))))

(fn SetSimulatePhysics
  (params (bSimulate :type Boolean))
  (Physics|SetSimulatePhysics (Variables|Default|GetStaticMesh) bSimulate))

(fn GetWorldRotation
  (return (Transformation|GetWorldRotation (Variables|Default|GetStaticMesh))))

(fn SetContinuousActionsRunning
  (params (Should%20Run :type Boolean) (InputValue :type Float%20%28double-precision%29) (Input%20Action%20Guid :type Guid%20Structure%20%28by%20ref%29))
  (for _array_element (Variables|Actions|GetContinuousActions)
    (Default|SetActionRunnin _array_element Should%20Run InputValue Input%20Action%20Guid)))

(fn RecalculateActions
  (Utilities|FlowControl|Sequence
    (:then_0
      (Utilities|Array|Clear (Variables|Actions|GetContinuousActions))
      (for _array_element (Actor|GetComponentsByClass "/Game/Blueprints/BuildParts/BuildPartActions/ContinuousBuildPartAction.ContinuousBuildPartAction_C")
        (Utilities|Array|Add (Variables|Actions|GetContinuousActions) _array_element)))
    (:then_1
      (Utilities|Array|Clear (Variables|Actions|GetInstantActions))
      (for _array_element_2 (Actor|GetComponentsByClass "/Game/Blueprints/BuildParts/BuildPartActions/InstantBuildPartAction.InstantBuildPartAction_C")
        (Utilities|Array|Add (Variables|Actions|GetInstantActions) _array_element_2)))))

(fn PerformInstantActions
  (params (InputValue :type Float%20%28double-precision%29))
  (for _array_element (Variables|Actions|GetInstantActions)
    (Default|PerformActionOnce _array_element InputValue)))

(fn AddConnectionSlotsGrid
  (params (Num%20X :type Integer) (Num%20Y :type Integer) (Z%20offset :type Float%20%28double-precision%29) (Slot%20Type :type BuildPartConnectionSlotType%20Enum :default "NewEnumerator0"))
  (if (not (or (<= Num%20X 0) (<= Num%20Y 0)))
    (for _index (range 0 (- Num%20X 1))
      (LocalVariables|SetX%20index _index)
      (for _index_2 (range 0 (- Num%20Y 1))
        (LocalVariables|SetY%20Index _index_2)
        (bind _returnvalue (Game|AddComponentbyClass "/Game/Blueprints/BuildParts/BuildPartConnectionSlot.BuildPartConnectionSlot_C" false (Math|Transform|MakeTransform (Math|Vector|MakeVector (+ (* (/ (* (LocalVariables|GetX%20size) (- Num%20X 1)) 2.0) -1.0) (* (LocalVariables|GetX%20index) (LocalVariables|GetX%20size))) (+ (* (/ (* (LocalVariables|GetY%20size) (- Num%20Y 1)) 2.0) -1.0) (* (LocalVariables|GetY%20Index) (LocalVariables|GetY%20size))) Z%20offset))))
        (Variables|/Game/Blueprints/BuildParts/BuildPartConnectionSlot.BuildPartConnectionSlot_C|SetConnectionSlotType _returnvalue Slot%20Type)))))

(fn AddConnectionSlotsOffset
  (params (Num%20X :type Integer) (Num%20Y :type Integer) (X%20offset :type Float%20%28double-precision%29) (Y%20offset :type Float%20%28double-precision%29) (Z%20offset :type Float%20%28double-precision%29) (Slot%20Type :type BuildPartConnectionSlotType%20Enum :default "NewEnumerator0"))
  (if (not (or (<= Num%20X 0) (<= Num%20Y 0)))
    (for _index (range 0 (- Num%20X 1))
      (LocalVariables|SetX%20index _index)
      (for _index_2 (range 0 (- Num%20Y 1))
        (LocalVariables|SetY%20Index _index_2)
        (bind _returnvalue (Game|AddComponentbyClass "/Game/Blueprints/BuildParts/BuildPartConnectionSlot.BuildPartConnectionSlot_C" false (Math|Transform|MakeTransform (Math|Vector|MakeVector (+ (* (/ (* (LocalVariables|GetX%20size) (- Num%20X 1)) 2.0) -1.0) (* (LocalVariables|GetX%20index) (LocalVariables|GetX%20size)) X%20offset) (+ (* (/ (* (LocalVariables|GetY%20size) (- Num%20Y 1)) 2.0) -1.0) (* (LocalVariables|GetY%20Index) (LocalVariables|GetY%20size)) Y%20offset) Z%20offset))))
        (Variables|/Game/Blueprints/BuildParts/BuildPartConnectionSlot.BuildPartConnectionSlot_C|SetConnectionSlotType _returnvalue Slot%20Type)))))

(fn GetGuid
  (if (not (== (.Guid (Utilities|Struct|BreakBuildPartInstanceData (Utilities|Struct|MakeBuildPartInstanceData "00000000000000000000000000000000" "None"))) (.Guid (Utilities|Struct|BreakBuildPartInstanceData (Variables|Data|GetBuildPartInstanceData)))))
    _
    (else
      (Utilities|Struct|SetmembersinBuildPartInstanceData (Variables|Data|GetBuildPartInstanceData) (Guid|NewGuid))))
  (return (.Guid (Utilities|Struct|BreakBuildPartInstanceData (Variables|Data|GetBuildPartInstanceData)))))

(fn GetBuildPartClass
  (if (Utilities|IsValidClass (Variables|Default|GetBuildPartClass))
    _
    (else
      (bind _returnvalue (Utilities|GetDataTableRow "/Game/Blueprints/BuildParts/BuildParts/BuildParts.BuildParts" (.BuildPartRowName (Utilities|Struct|BreakBuildPartInstanceData (Variables|Data|GetBuildPartInstanceData))))
        (:then
          (Variables|Default|SetBuildPartClass (.Class (Utilities|Struct|BreakBuildPartData _returnvalue))))
        (:RowNotFound
          _))))
  (return (Variables|Default|GetBuildPartClass)))

(fn GetBuildPartInstanceData
  (return (Variables|Data|GetBuildPartInstanceData)))

(fn GetParentBuildAssembly
  (Utilities|IsValid (Variables|Default|GetBuildAssemblyPawn)
    (:Is%20Valid
      _)
    (:Is%20Not%20Valid
      (bind _asbuild_assembly_pawn (Utilities|Casting|CastToBuildAssemblyPawn (Actor|GetAttachParentActor))
        (:then
          (Variables|Default|SetBuildAssemblyPawn _asbuild_assembly_pawn))
        (:CastFailed
          _))))
  (return (Variables|Default|GetBuildAssemblyPawn)))

(fn RevertInstanceData
  (params (PreviousBuildPartInstanceData :type Build%20Part%20Instance%20Data%20Structure))
  (Variables|Data|SetBuildPartInstanceData PreviousBuildPartInstanceData)
  (LocationAndRotation|UpdateBuildPartRelativeLocation))

(fn SetStabilityControlData
  (params (StabilityControlInstanceData :type Stability%20Control%20Instance%20Data%20Structure))
  (bind (_pitchpositivebuildpartguid _pitchnegativebuildpartguid _rollpositivebuildpartguid _rollnegativebuildpartguid _magnitudefactor) (Utilities|Struct|BreakStabilityControlInstanceData StabilityControlInstanceData))
  (bind _buildpartinstancedata (Variables|Data|GetBuildPartInstanceData))
  (bind _stabilitycontrolinstancedata (Utilities|Struct|BreakBuildPartInstanceData _buildpartinstancedata))
  (bind (_pitchpositivebuildpartguid_2 _pitchnegativebuildpartguid_2 _rollpositivebuildpartguid_2 _rollnegativebuildpartguid_2 _magnitudefactor_2) (Utilities|Struct|BreakStabilityControlInstanceData _stabilitycontrolinstancedata))
  (if (Math|Boolean|ORBoolean (!= _pitchpositivebuildpartguid _pitchpositivebuildpartguid_2) (!= _pitchnegativebuildpartguid _pitchnegativebuildpartguid_2) (!= _rollpositivebuildpartguid _rollpositivebuildpartguid_2) (!= _rollnegativebuildpartguid _rollnegativebuildpartguid_2) (!= _magnitudefactor _magnitudefactor_2))
    (Utilities|Struct|SetmembersinBuildPartInstanceData _buildpartinstancedata StabilityControlInstanceData)
    (Default|CallBuildPartModified)))

(fn SelectBuildPart)

(fn ConnectSlots
  (for _array_element (Variables|ConnectionSlots|GetFemaleUnconnectedSlots)
    (Default|FindConnectedSlot _array_element))
  (for _array_element_2 (Variables|ConnectionSlots|GetMaleUnconnectedSlots)
    (Default|FindConnectedSlot _array_element_2)))

(fn DisconnectAllSlots
  (for _array_element (Actor|GetComponentsByClass "/Game/Blueprints/BuildParts/BuildPartConnectionSlot.BuildPartConnectionSlot_C")
    (Default|DisconnectSlot _array_element))
  (ConnectionSlots|RecalculateConnectionSlots))