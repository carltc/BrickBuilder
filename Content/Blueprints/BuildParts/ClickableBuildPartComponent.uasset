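; Component that makes its owning BuildPart selectable and highlightable by mouse in build play.
; When clickable, it binds the part's click and cursor-over events, filtered by whether the part can be built with or moved.
; Left clicks toggle selection or place the selected part through the BuildPlayGameMode, depending on its mouse mode.
; Hover and selection highlights use custom depth with separate stencil values on the part's static mesh.
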(event Custom|OnMouseClick
  (params (TouchedActor :type Actor%20Object%20Reference) (ButtonPressed :type Key%20Structure :default "None"))
  (bind _buildplaygamemode (CallFunction|GetBuildPlayGameMode))
  (bind _buildpartref (Variables|Default|GetBuildPartRef))
  ;[1 1 1] On Mouse Click
  (if (== ButtonPressed "LeftMouseButton")
    (Utilities|IsValid _buildpartref
      (:Is%20Valid
        (if (and (Variables|/Game/Blueprints/BuildParts/BuildPart.BuildPart_C|GetCanBeMoved _buildpartref) (.CanBuildWith (Utilities|Struct|BreakBuildPartData (Variables|/Game/Blueprints/BuildParts/BuildPart.BuildPart_C|GetBuildPartData _buildpartref))))
          (switch Utilities|FlowControl|Switch|SwitchonBuildPlayMouseMode (Variables|/Game/Blueprints/BuildPlayMode/BuildPlayGameMode.BuildPlayGameMode_C|GetBuildPlayMouseMode (CallFunction|GetBuildPlayGameMode))
            (:NewEnumerator0
              (CallFunction|SetSelected (not (Variables|Default|GetIsSelected)))
              (if (Variables|Default|GetIsSelected)
                (Default|SetSelectedBuildPart _buildplaygamemode (Variables|Default|GetBuildPartRef))
                (else
                  (Default|SetSelectedBuildPart _buildplaygamemode))))
            (:NewEnumerator1
              (if (Variables|Default|GetIsSelected)
                (Default|PlaceSelectedBuildPart _buildplaygamemode)))))))))

(event Custom|OnMouseHoverBegin
  (params (TouchedActor :type Actor%20Object%20Reference))
  (bind _buildpartref (Variables|Default|GetBuildPartRef))
  ;[1 1 1] On Mouse Hover
  (Variables|Default|SetIsHovered true)
  (Utilities|IsValid _buildpartref
    (:Is%20Valid
      (if (.CanBuildWith (Utilities|Struct|BreakBuildPartData (Variables|/Game/Blueprints/BuildParts/BuildPart.BuildPart_C|GetBuildPartData _buildpartref)))
        (switch Utilities|FlowControl|Switch|SwitchonBuildPlayMouseMode (Variables|/Game/Blueprints/BuildPlayMode/BuildPlayGameMode.BuildPlayGameMode_C|GetBuildPlayMouseMode (CallFunction|GetBuildPlayGameMode))
          (:NewEnumerator0
            (CallFunction|SetHovered (Variables|Default|GetIsHovered))))))))

(event Custom|OnMouseHoverEnd
  (params (TouchedActor :type Actor%20Object%20Reference))
  (bind _buildpartref (Variables|Default|GetBuildPartRef))
  ;[1 1 1] On Mouse Hover
  (Variables|Default|SetIsHovered false)
  (Utilities|IsValid _buildpartref
    (:Is%20Valid
      (if (.CanBuildWith (Utilities|Struct|BreakBuildPartData (Variables|/Game/Blueprints/BuildParts/BuildPart.BuildPart_C|GetBuildPartData _buildpartref)))
        (switch Utilities|FlowControl|Switch|SwitchonBuildPlayMouseMode (Variables|/Game/Blueprints/BuildPlayMode/BuildPlayGameMode.BuildPlayGameMode_C|GetBuildPlayMouseMode (CallFunction|GetBuildPlayGameMode))
          (:NewEnumerator0
            (CallFunction|SetHovered (Variables|Default|GetIsHovered))))))))

(event Custom|Initialise%20Clickableness
  (if (Variables|Default|GetIsClickable)
    (bind _asbuild_part (Utilities|Casting|CastToBuildPart (Components|GetOwner)))
    (bind _output_get (Variables|Default|SetBuildPartRef _asbuild_part))
    (Utilities|FlowControl|Sequence
      (:then_0
        ;[1 1 1] On Mouse Click
        (EventDispatchers|BindEventtoOnClicked _output_get (delegate Custom|OnMouseClick)))
      (:then_1
        ;[1 1 1] On Mouse Hover
        (EventDispatchers|BindEventtoOnBeginCursorOver _output_get (delegate Custom|OnMouseHoverBegin)))
      (:then_2
        (EventDispatchers|BindEventtoOnEndCursorOver _output_get (delegate Custom|OnMouseHoverEnd))))))

(event EventBeginPlay
  (CallFunction|InitialiseClickableness))

(fn SetIsClickable
  (Variables|Default|SetIsClickable true)
  (CallFunction|InitialiseClickableness))

(fn GetBuildPlayGameMode
  (Utilities|IsValid (Variables|Default|GetBuildPlayGameMode)
    (:Is%20Valid
      _)
    (:Is%20Not%20Valid
      (bind _asbuild_play_game_mode (Utilities|Casting|CastToBuildPlayGameMode (Game|GetGameMode))
        (:then
          (Variables|Default|SetBuildPlayGameMode _asbuild_play_game_mode))
        (:CastFailed
          _))))
  (return (Variables|Default|GetBuildPlayGameMode)))

(fn SetHovered
  (params (IsHovered :type Boolean))
  (bind _buildpartref (Variables|Default|GetBuildPartRef))
  (bind _staticmesh (Variables|/Game/Blueprints/BuildParts/BuildPart.BuildPart_C|GetStaticMesh _buildpartref))
  (if (and (.CanBuildWith (Utilities|Struct|BreakBuildPartData (Variables|/Game/Blueprints/BuildParts/BuildPart.BuildPart_C|GetBuildPartData (Variables|Default|GetBuildPartRef)))) (not (Variables|Default|GetIsSelected)))
    (bind _output_get (Variables|Default|SetIsHovered IsHovered))
    (Rendering|SetRenderCustomDepth _staticmesh _output_get)
    (Rendering|SetCustomDepthStencilValue _staticmesh 1)))

(fn SetSelected
  (params (IsSelected :type Boolean))
  (bind _buildpartref (Variables|Default|GetBuildPartRef))
  (bind _staticmesh (Variables|/Game/Blueprints/BuildParts/BuildPart.BuildPart_C|GetStaticMesh _buildpartref))
  (if (and (.CanBuildWith (Utilities|Struct|BreakBuildPartData (Variables|/Game/Blueprints/BuildParts/BuildPart.BuildPart_C|GetBuildPartData (Variables|Default|GetBuildPartRef)))) (Variables|/Game/Blueprints/BuildParts/BuildPart.BuildPart_C|GetCanBeMoved (Variables|Default|GetBuildPartRef)))
    (bind _output_get (Variables|Default|SetIsSelected IsSelected))
    (Rendering|SetRenderCustomDepth _staticmesh _output_get)
    (Rendering|SetCustomDepthStencilValue _staticmesh 0)))