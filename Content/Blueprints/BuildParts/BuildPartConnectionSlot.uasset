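; Connection slot component on a BuildPart that links to a slot on another part in the brick-building game.
; AttemptToConnect runs a component overlap query, ignoring its own part, and links both ways with the first slot found.
; DisconnectSlot clears both sides and fires Disconnected on each, while getters expose the linked slot and part.
; Tick draws a debug sphere when the game instance enables debug; the Male/Female shape drawing is unreachable.
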(event EventTick
  (params (DeltaSeconds :type Float%20%28single-precision%29))
  (if (Variables|/Game/Blueprints/BrickBuilderGameInstance.BrickBuilderGameInstance_C|GetShowDebug (CallFunction|GetBrickBuilderGameInstance))
    (Rendering|Debug|DrawDebugSphere (Transformation|GetWorldLocation) 1.0 12 "(R=1.000000,G=0.000000,B=0.000000,A=1.000000)" 0.0 1.0)))

(fn GetBrickBuilderGameInstance
  (Utilities|IsValid (Variables|Game|GetBrickBuilderGameInstance)
    (:Is%20Valid
      _)
    (:Is%20Not%20Valid
      (bind _asbrick_builder_game_instance (Utilities|Casting|CastToBrickBuilderGameInstance (Game|GetGameInstance))
        (:then
          (Variables|Game|SetBrickBuilderGameInstance _asbrick_builder_game_instance))
        (:CastFailed
          _))))
  (return (Variables|Game|GetBrickBuilderGameInstance)))

(fn IsConnected
  (return (Utilities|IsValid (Variables|Default|GetConnectedSlot))))

(fn ConnectSlot
  (params (ConnectedSlot :type Build%20Part%20Connection%20Slot%20Object%20Reference))
  (if (not (CallFunction|IsConnected))
    (Variables|Default|SetConnectedSlot ConnectedSlot)
    (Default|CallConnected self)))

(fn GetParentBuildPart
  (Utilities|IsValid (Variables|Game|GetParentBuildPart)
    (:Is%20Valid
      _)
    (:Is%20Not%20Valid
      (bind _asbuild_part (Utilities|Casting|CastToBuildPart (Components|GetOwner))
        (:then
          (Variables|Game|SetParentBuildPart _asbuild_part))
        (:CastFailed
          _))))
  (return (Variables|Game|GetParentBuildPart)))

(fn AttempttoConnect
  (bind _self self)
  (bind _self_2 self)
  (bind (_outcomponents _returnvalue) (Class|KismetSystemLibrary|ComponentOverlapComponents _self_2 (Transformation|GetWorldTransform _self_2) (Utilities|Array|MakeArray "ObjectTypeQuery7") "BuildPartConnectionSlot_C" (Utilities|Array|MakeArray (CallFunction|GetParentBuildPart))))
  (if _returnvalue
    (bind _asbuild_part_connection_slot (Utilities|Casting|CastToBuildPartConnectionSlot (Utilities|Array|Get(acopy) _outcomponents))
      (:then
        (Utilities|FlowControl|Sequence
          (:then_0
            (CallFunction|ConnectSlot _self _asbuild_part_connection_slot))
          (:then_1
            (CallFunction|ConnectSlot _asbuild_part_connection_slot _self))
          (:then_2
            (return true))))
      (:CastFailed
        (return false)))
    (else
      (return false))))

(fn DisconnectSlot
  (bind _self self)
  (if (CallFunction|IsConnected)
    (LocalVariables|SetPreviouslyConnectedSlot (Variables|Default|GetConnectedSlot))
    (Variables|Default|SetConnectedSlot 0)
    (Variables|BuildPartConnectionSlot_C|SetConnectedSlot (LocalVariables|GetPreviouslyConnectedSlot) 0)
    (Default|CallDisconnected _self _self (LocalVariables|GetPreviouslyConnectedSlot))
    (Default|CallDisconnected (LocalVariables|GetPreviouslyConnectedSlot) (LocalVariables|GetPreviouslyConnectedSlot) self)))

(fn GetConnectedBuildPart
  (if (CallFunction|IsConnected)
    (return (CallFunction|GetParentBuildPart (Variables|Default|GetConnectedSlot)))
    (else
      (return 0))))

(fn GetConnectedSlot
  (return (Variables|Default|GetConnectedSlot)))