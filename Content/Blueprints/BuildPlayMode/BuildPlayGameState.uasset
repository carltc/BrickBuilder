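; BuildPlayGameState is a game state Blueprint that holds shared selection data for build-play mode.
; Getter and setter pairs expose the current build part, its class, its connection slot and the selected connection slot.
; A connection slot seed counter can be read and incremented by one.
; It has no active event logic, acting purely as a state store for other Blueprints.
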(event EventBeginPlay)

(event EventTick
  (params (DeltaSeconds :type Float%20%28single-precision%29)))

(fn ConstructionScript)

(fn SetCurrentBuildPart
  (params (NewBuildPart :type Build%20Part%20Object%20Reference))
  (Variables|Builder|SetCurrentBuildPart NewBuildPart))

(fn GetCurrentBuildPart
  (return (Variables|Builder|GetCurrentBuildPart)))

(fn GetSelectedConnectionSlot
  (return (Variables|Builder|GetSelectedConnectionSlot)))

(fn SetSelectedConnectionSlot
  (params (SelectedConnectionSlot :type Build%20Part%20Connection%20Slot%20Object%20Reference))
  (Variables|Builder|SetSelectedConnectionSlot SelectedConnectionSlot))

(fn GetCurrentBuildPartConnectionSlot
  (return (Variables|Builder|GetCurrentBuildPartConnectionSlot)))

(fn SetCurrentBuildPartConnectionSlot
  (params (CurrentBuildPartConnectionSlot :type Build%20Part%20Connection%20Slot%20Object%20Reference))
  (Variables|Builder|SetCurrentBuildPartConnectionSlot CurrentBuildPartConnectionSlot))

(fn GetCurrentBuildPartClass
  (return (Variables|Default|GetCurrentBuildPartClass)))

(fn SetCurrentBuildPartClass
  (params (CurrentBuildPartClass :type Build%20Part%20Class%20Reference))
  (Variables|Default|SetCurrentBuildPartClass CurrentBuildPartClass))

(fn IncrementConnectionSlotSeed
  (Variables|Default|SetConnectionSlotSeed (+ (Variables|Default|GetConnectionSlotSeed) 1)))

(fn GetConnectionSlotSeed
  (return (Variables|Default|GetConnectionSlotSeed)))