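; Game mode for a brick-building game that switches between Build and Play modes, swapping the UI and toggling whether the assembly operates.
; At start it spawns saved assemblies from save games and possesses one, creating a starter-brick assembly if none exist.
; In Build mode, a mouse-mode state drives selecting, moving and deleting parts.
; Moved parts snap to connection slots with their descendants, use overlap checks for validity, and can revert from cached instance data.
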(event Custom|BuildAssemblyChangedEvent
  (params (NewBuildAssemblyPawn :type Build%20Assembly%20Pawn%20Object%20Reference))
  (bind _buildmodeui (Variables|UI|GetBuildModeUI))
  ;[1 1 1] Begin Play
  (Utilities|IsValid _buildmodeui
    (:Is%20Valid
      (Default|CallBuildAssemblyChanged _buildmodeui NewBuildAssemblyPawn))))

(event Custom|SelectedBuildPartChangedEvent
  (params (NewBuildPart :type Build%20Part%20Object%20Reference))
  (bind _buildmodeui (Variables|UI|GetBuildModeUI))
  ;[1 1 1] Begin Play
  (Utilities|IsValid _buildmodeui
    (:Is%20Valid
      (Default|CallSelectedBuildPartChanged _buildmodeui NewBuildPart))))

(event EventBeginPlay
  (bind _returnvalue (Game|GetPlayerController 0))
  ;[1 1 1] Begin Play
  (Utilities|FlowControl|Sequence
    (:then_0
      (Variables|/Script/Engine.PlayerController|SetbShowMouseCursor _returnvalue true)
      (Input|SetInputModeGameandUI _returnvalue 0 "DoNotLock" false false)
      (EventDispatchers|BindEventtoBuildAssemblyPawnChanged (delegate Custom|BuildAssemblyChangedEvent))
      (EventDispatchers|BindEventtoSelectedBuildPartChanged (delegate Custom|SelectedBuildPartChangedEvent)))
    (:then_1
      (BuildAssembly|LoadBuildAssemblies)
      (BuildAssembly|PossesBuildAssembly (BuildAssembly|GetBuildAssemblyPawn)))
    (:then_2
      (Modes|SetBuildPlayMode "NewEnumerator0"))
    (:then_3
      (Default|SetBaseLocation (BuildAssembly|GetBuildAssemblyPawn) "0.000000,0.000000,100.000000"))))

(event EventTick
  (params (DeltaSeconds :type Float%20%28single-precision%29))
  ;[1 1 1] TICK
  (switch Utilities|FlowControl|Switch|SwitchonBuildPlayMode (Modes|GetBuildPlayMode)
    (:NewEnumerator0
      (switch Utilities|FlowControl|Switch|SwitchonBuildPlayMouseMode (Variables|Modes|GetBuildPlayMouseMode)
        (:NewEnumerator1
          (BuildParts|MoveFirstSelectedBuildParttoNearestValidConnectionSlot))))))

(fn ConstructionScript)

(fn SpawnBuildPartinAssembly
  (params (Build%20Part%20Class :type Build%20Part%20Class%20Reference) (Location :type Vector) (CanBeMoved :type Boolean))
  (bind (_row_name _build_part_data _found_) (BuildParts|GetBuildPartData Build%20Part%20Class))
  (if _found_
    (bind _returnvalue (Game|SpawnActorfromClass Build%20Part%20Class (Math|Transform|MakeTransform Location) "Undefined" "MultiplyWithRoot" (Game|GetPlayerController 0) (Utilities|Struct|MakeBuildPartInstanceData "00000000000000000000000000000000" _row_name 0 "0.000000,0.000000,0.000000" "0.000000,0.000000,0.000000" "0.000000,0.000000,0.000000" "0.000000,0.000000,0.000000" CanBeMoved) CanBeMoved 0))
    (AddComponent|AddClickableBuildPartComponent _returnvalue true)
    (BuildAssembly|AddBuildParttoAssembly _returnvalue)
    (BuildParts|AddSelectedBuildPart _returnvalue false)
    (BuildParts|PickUpBuildPart _returnvalue)
    (return _returnvalue)))

(fn GetBuildPlayPlayerController
  (Utilities|IsValid (Variables|Game|GetBuildPlayPlayerController)
    (:Is%20Valid
      _)
    (:Is%20Not%20Valid
      (bind _asbuild_play_player_controller (Utilities|Casting|CastToBuildPlayPlayerController (Game|GetPlayerController 0))
        (:then
          (Variables|Game|SetBuildPlayPlayerController _asbuild_play_player_controller))
        (:CastFailed
          _))))
  (return (Variables|Game|GetBuildPlayPlayerController)))

(fn GetBuildPlayGameState
  (Utilities|IsValid (Variables|Game|GetBuildPlayGameState)
    (:Is%20Valid
      _)
    (:Is%20Not%20Valid
      (bind _asbuild_play_game_state (Utilities|Casting|CastToBuildPlayGameState (Game|GetGameState))
        (:then
          (Variables|Game|SetBuildPlayGameState _asbuild_play_game_state))
        (:CastFailed
          _))))
  (return (Variables|Game|GetBuildPlayGameState)))

(fn AddBuildParttoAssembly
  (params (Build%20Part :type Build%20Part%20Object%20Reference))
  (bind _buildassemblypawn (BuildAssembly|GetBuildAssemblyPawn))
  (Utilities|IsValid _buildassemblypawn
    (:Is%20Valid
      (Default|AddBuildPart _buildassemblypawn Build%20Part false))))

(fn SpawnBuildPartbyClass
  (params (New%20Build%20Part%20Class :type Build%20Part%20Class%20Reference))
  (BuildParts|SpawnBuildPartinAssembly New%20Build%20Part%20Class "0, 0, 0" true))

(fn ApplyBuildPlayMode
  (switch Utilities|FlowControl|Switch|SwitchonBuildPlayMode (Variables|Modes|GetBuildPlayMode)
    (:NewEnumerator0
      (Modes|ApplyBuildMode)
      (Modes|SetBuildPlayMouseMode "NewEnumerator0"))
    (:NewEnumerator1
      (Modes|ApplyPlayMode)
      (Modes|SetBuildPlayMouseMode "NewEnumerator2"))))

(fn ApplyBuildMode
  (Utilities|FlowControl|Sequence
    (:then_0
      (BuildAssembly|BuildAssemblyBuildModeBegin))
    (:then_1
      (UI|ClearViewportUIs)
      (Utilities|IsValid (Variables|UI|GetBuildModeUI)
        (:Is%20Valid
          _)
        (:Is%20Not%20Valid
          (bind _returnvalue (UserInterface|CreateWidget "/Game/UI/BuildPlay/Build/BuildModeUI.BuildModeUI_C" (Game|GetBuildPlayPlayerController)))
          (bind _output_get (Variables|UI|SetBuildModeUI _returnvalue))
          (Default|CallBuildAssemblyChanged _output_get (BuildAssembly|GetBuildAssemblyPawn))))
      (UserInterface|Viewport|AddtoViewport (Variables|UI|GetBuildModeUI) 0))))

(fn ClearViewportUIs
  (Viewport|RemoveAllWidgets))

(fn ApplyPlayMode
  (Utilities|FlowControl|Sequence
    (:then_0
      (BuildAssembly|BuildAssemblyPlayModeBegin)
      (BuildParts|UnselectAllSelectedBuildParts))
    (:then_1
      (UI|ClearViewportUIs)
      (Utilities|IsValid (Variables|UI|GetPlayModeUI)
        (:Is%20Valid
          _)
        (:Is%20Not%20Valid
          (bind _returnvalue (UserInterface|CreateWidget "/Game/UI/BuildPlay/Play/PlayModeUI.PlayModeUI_C" (Game|GetBuildPlayPlayerController)))
          (Variables|UI|SetPlayModeUI _returnvalue)))
      (UserInterface|Viewport|AddtoViewport (Variables|UI|GetPlayModeUI) 0))))

(fn BuildAssemblyPlayModeBegin
  (Default|SetBuildAssemblyOperating (BuildAssembly|GetBuildAssemblyPawn) true))

(fn BuildAssemblyBuildModeBegin
  (Default|SetBuildAssemblyOperating (BuildAssembly|GetBuildAssemblyPawn) false))

(fn SetBuildPlayMode
  (params (BuildPlayMode :type BuildPlayMode%20Enum :default "NewEnumerator0"))
  (Variables|Modes|SetBuildPlayMode BuildPlayMode)
  (Modes|ApplyBuildPlayMode))

(fn GetBuildAssemblyPawn
  (bind _returnvalue (Game|Player|GetPlayerPawn 0))
  (Utilities|IsValid (Variables|Game|GetBuildAssemblyPawn)
    (:Is%20Valid
      _)
    (:Is%20Not%20Valid
      (Utilities|IsValid _returnvalue
        (:Is%20Valid
          (bind _asbuild_assembly_pawn (Utilities|Casting|CastToBuildAssemblyPawn _returnvalue)
            (:then
              (Variables|Game|SetBuildAssemblyPawn _asbuild_assembly_pawn))
            (:CastFailed
              (if (> (Utilities|Map|Length (Variables|BuildAssemblies|GetBuildAssemblies)) 0) :!label _label
                (bind _values (Utilities|Map|Values (Variables|BuildAssemblies|GetBuildAssemblies)))
                (if (.ReturnValue (Utilities|Map|Find (Variables|BuildAssemblies|GetBuildAssemblies) (Default|GetGuid (Utilities|Array|Get(acopy) _values (Utilities|Array|LastIndex _values)))))
                  (Variables|Game|SetBuildAssemblyPawn (.Value (Utilities|Map|Find (Variables|BuildAssemblies|GetBuildAssemblies) (Default|GetGuid (Utilities|Array|Get(acopy) _values (Utilities|Array|LastIndex _values))))))
                  (else
                    (bind _build_assembly (BuildAssembly|SpawnNewBuildAssembly :!label _label_2))
                    (Variables|Game|SetBuildAssemblyPawn _build_assembly)))
                (else
                  (goto _label_2))))))
        (:Is%20Not%20Valid
          (goto _label)))))
  (return (Variables|Game|GetBuildAssemblyPawn)))

(fn SpawnBuildAssemblyPawn
  (params (BuildAssemblyInstanceData :type Build%20Assembly%20Instance%20Data%20Structure))
  (bind _returnvalue (Game|SpawnActorfromClass "/Game/Blueprints/BuildAssembly/BuildAssemblyPawn.BuildAssemblyPawn_C" (Math|Transform|MakeTransform (.BaseLocation (Utilities|Struct|BreakBuildAssemblyInstanceData BuildAssemblyInstanceData))) "Undefined" "MultiplyWithRoot" 0 BuildAssemblyInstanceData 0))
  (Utilities|Map|Add (Variables|BuildAssemblies|GetBuildAssemblies) (Default|GetGuid _returnvalue) _returnvalue)
  (return _returnvalue))

(fn GetBuildPlayMode
  (return (Variables|Modes|GetBuildPlayMode)))

(fn LoadBuildAssemblies
  (bind _foundfiles (Class|BlueprintFileUtilsBPLibrary|FindFiles (Utilities|String|Append (Class|KismetSystemLibrary|GetProjectSavedDirectory) "SaveGames/")))
  (for _array_element _foundfiles
    (if (.ReturnValue (Utilities|String|Split _array_element "."))
      (bind _returnvalue (SaveGame|DoesSaveGameExist (.LeftS (Utilities|String|Split _array_element "."))))
      (if _returnvalue
        (bind _returnvalue_2 (SaveGame|LoadGamefromSlot (.LeftS (Utilities|String|Split _array_element "."))))
        (bind _asbuild_assembly_save (Utilities|Casting|CastToBuildAssemblySave _returnvalue_2))
        (LocalVariables|SetCurrentBuildAssemblyInstanceData (Variables|/Game/Blueprints/Saving/BuildAssemblySave.BuildAssemblySave_C|GetBuildAssemblyInstanceData _asbuild_assembly_save))
        (if (Utilities|Operators|EqualEqual (.BaseLocation (Utilities|Struct|BreakBuildAssemblyInstanceData (Variables|/Game/Blueprints/Saving/BuildAssemblySave.BuildAssemblySave_C|GetBuildAssemblyInstanceData _asbuild_assembly_save))) "0.000000,0.000000,100.000000" 1.0)
          (bind _structout (Utilities|Struct|SetmembersinBuildAssemblyInstanceData (LocalVariables|GetCurrentBuildAssemblyInstanceData) (BuildAssembly|GetRandomBuildAssemblyLocation)))
          (LocalVariables|SetCurrentBuildAssemblyInstanceData _structout))
        (bind _build_assembly (BuildAssembly|SpawnBuildAssemblyPawn (LocalVariables|GetCurrentBuildAssemblyInstanceData)))
        (Default|LoadBuildParts _build_assembly (Variables|/Game/Blueprints/Saving/BuildAssemblySave.BuildAssemblySave_C|GetBuildPartsInstanceData _asbuild_assembly_save))
        (BuildAssembly|MakeBuildAssemblyClickable _build_assembly)))))

(fn GetRandomBuildAssemblyLocation
  (bind _returnvalue (Math|Float|MakeLiteralFloat 5e+02))
  (bind _returnvalue_2 (* _returnvalue -1.0))
  (return (Math|Vector|MakeVector (Math|Random|RandomFloatinRange _returnvalue_2 _returnvalue) (Math|Random|RandomFloatinRange _returnvalue_2 _returnvalue) 1e+02)))

(fn PossesBuildAssembly
  (params (BuildAssemblyPawn :type Build%20Assembly%20Pawn%20Object%20Reference))
  (Pawn|Possess (Game|GetBuildPlayPlayerController) BuildAssemblyPawn)
  (Variables|Game|SetBuildAssemblyPawn BuildAssemblyPawn)
  (Default|CallBuildAssemblyPawnChanged BuildAssemblyPawn))

(fn SpawnNewBuildAssembly
  (bind _build_assembly (BuildAssembly|SpawnBuildAssemblyPawn (Utilities|Struct|MakeBuildAssemblyInstanceData "00000000000000000000000000000000" (BuildAssembly|GetRandomBuildAssemblyLocation) "" "()")))
  (BuildAssembly|PossesBuildAssembly _build_assembly)
  (BuildParts|SpawnBuildPartinAssembly "/Game/Blueprints/BuildParts/BuildParts/Bricks/BP_Brick_2x2.BP_Brick_2x2_C" "0, 0, 0" false)
  (return _build_assembly))

(fn SetBuildPlayMouseMode
  (params (BuildPlayMouseMode :type BuildPlayMouseMode%20Enum :default "NewEnumerator0"))
  (switch Utilities|FlowControl|Switch|SwitchonBuildPlayMouseMode BuildPlayMouseMode
    (:NewEnumerator0
      _)
    (:NewEnumerator1
      (if (CallFunction|AnyBuildPartsSelected)
        _
        (else
          (return false))))
    (:NewEnumerator3
      (BuildParts|UnselectAllSelectedBuildParts :!label _label))
    (:NewEnumerator2
      (goto _label)))
  (Variables|Modes|SetBuildPlayMouseMode BuildPlayMouseMode)
  (return true))

(fn GetBuildPartData
  (params (BuildPartClass :type Build%20Part%20Class%20Reference))
  (bind _outrownames (DataTable|GetDataTableRowNames "/Game/Blueprints/BuildParts/BuildParts/BuildParts.BuildParts"))
  (for _array_element _outrownames
    (bind _returnvalue (Utilities|GetDataTableRow "/Game/Blueprints/BuildParts/BuildParts/BuildParts.BuildParts" _array_element)
      (:then
        (if (== (.Class (Utilities|Struct|BreakBuildPartData _returnvalue)) BuildPartClass)
          (return _array_element _returnvalue true)))))
  (return "None" "" false))

(fn UnselectAllSelectedBuildParts
  (for _array_element (BuildParts|GetSelectedBuildParts)
    (Utilities|IsValid _array_element
      (:Is%20Valid
        (BuildParts|UnselectBuildPart _array_element))))
  (Utilities|Array|Clear (Variables|BuildParts|GetSelectedBuildParts))
  (Utilities|Map|Clear (Variables|Data|GetPreviousBuildPartInstanceDatas)))

(fn RevertOperation
  (switch Utilities|FlowControl|Switch|SwitchonBuildPlayMode (Modes|GetBuildPlayMode)
    (:NewEnumerator0
      (switch Utilities|FlowControl|Switch|SwitchonBuildPlayMouseMode (Variables|Modes|GetBuildPlayMouseMode)
        (:NewEnumerator1
          (CallFunction|RevertBuildPartInstanceData)
          (Modes|SetBuildPlayMouseMode "NewEnumerator0"))))))

(fn AddSelectedBuildPart
  (params (NewSelectedBuildPart :type Build%20Part%20Object%20Reference) (MultiSelect? :type Boolean))
  (if MultiSelect?
    _
    (else
      (BuildParts|UnselectAllSelectedBuildParts)))
  (Utilities|IsValid NewSelectedBuildPart
    (:Is%20Valid
      (bind _succeeded_ (Default|SetSelected (Actor|GetComponentbyClass NewSelectedBuildPart "/Game/Blueprints/BuildParts/ClickableBuildPartComponent.ClickableBuildPartComponent_C") true))
      (if _succeeded_
        (Utilities|Array|Add (Variables|BuildParts|GetSelectedBuildParts) NewSelectedBuildPart)
        (Utilities|Map|Add (Variables|Data|GetPreviousBuildPartInstanceDatas) NewSelectedBuildPart (|Copy (Default|GetBuildPartInstanceData NewSelectedBuildPart)))
        (for _array_element (Default|GetDescendantBuildParts NewSelectedBuildPart)
          (Utilities|Map|Add (Variables|Data|GetPreviousBuildPartInstanceDatas) _array_element (|Copy (Default|GetBuildPartInstanceData _array_element))))
        (Default|CallSelectedBuildPartChanged NewSelectedBuildPart)))))

(fn PlaceBuildPart
  (params (Build%20Part%20To%20Place :type Build%20Part%20Object%20Reference))
  ;[1 1 1] Check if placement is valid
  (bind _is_valid (BuildParts|CheckValidBuildPartPlacements Build%20Part%20To%20Place))
  (if _is_valid
    ;[1 1 1] Set UI unselected
    (BuildParts|UnselectBuildPart Build%20Part%20To%20Place)
    ;[1 1 1] Set mode as not moving
    (Modes|SetBuildPlayMouseMode "NewEnumerator0")
    ;[1 1 1] Connect Build Parts To Assembly
    (Default|ConnectUnconnectedSlots Build%20Part%20To%20Place)
    ;[1 1 1] Call modified event
    (Default|CallBuildAssemblyModified (BuildAssembly|GetBuildAssemblyPawn) true)))

(fn PickUpBuildPart
  (params (Build%20Part%20To%20Pickup :type Build%20Part%20Object%20Reference))
  ;[1 1 1] Set mode as not moving
  (bind _set_ (Modes|SetBuildPlayMouseMode "NewEnumerator1"))
  (if _set_
    ;[1 1 1] Disconnect build part from assembly
    (Default|DisconnectNonChildSlots Build%20Part%20To%20Pickup)
    ;[1 1 1] Select this build part
    (BuildParts|AddSelectedBuildPart Build%20Part%20To%20Pickup false)))

(fn MoveFirstSelectedBuildParttoNearestValidConnectionSlot
  (bind _selectedbuildparts (BuildParts|GetSelectedBuildParts))
  (bind _selectedbuildparts_2 (BuildParts|GetSelectedBuildParts))
  (bind _asbuild_play_player_controller (Game|GetBuildPlayPlayerController))
  (bind _buildplaygamestate (Game|GetBuildPlayGameState))
  (bind _buildassemblypawn (BuildAssembly|GetBuildAssemblyPawn))
  (bind _selectedbuildparts_3 (BuildParts|GetSelectedBuildParts))
  (bind _selectedbuildparts_4 (BuildParts|GetSelectedBuildParts))
  (bind _connectionslotseed (Default|GetConnectionSlotSeed _buildplaygamestate))
  (bind _output (Utilities|Array|Get(acopy) _selectedbuildparts_3))
  (bind _output_2 (Utilities|Array|Get(acopy) _selectedbuildparts_4))
  (bind _output_3 (Utilities|Array|Get(acopy) _selectedbuildparts))
  (bind _output_4 (Utilities|Array|Get(acopy) _selectedbuildparts_2))
  (bind _thisanddescedantsbuildparts (Default|GetThisandDescendantBuildParts _output_4))
  (bind _array (Utilities|Array|MakeArray _output_2))
  (bind (_world_location _found_) (Default|GetWorldLocationUnderMouseCursor _asbuild_play_player_controller _array))
  (bind (_closestconnectionslot1 _found__2) (Default|GetNearestConnectionSlot _buildassemblypawn _world_location _thisanddescedantsbuildparts))
  (bind _connectionslottype (Variables|/Game/Blueprints/BuildParts/BuildPartConnectionSlot.BuildPartConnectionSlot_C|GetConnectionSlotType _closestconnectionslot1))
  (bind (_empty_socket_found _connectionslot) (Default|GetValidConnectionSlot _output_3 _connectionslottype _connectionslotseed))
  (Utilities|IsValid _output_2
    (:Is%20Valid
      (if _found_
        (if _found__2
          (if _empty_socket_found
            (Default|SetBuildPartLocation (BuildAssembly|GetBuildAssemblyPawn) (Utilities|Array|Get(acopy) (BuildParts|GetSelectedBuildParts)) _connectionslot _closestconnectionslot1)
            (BuildParts|MoveChildBuildParts _output)
            (bind _is_valid (BuildParts|CheckValidBuildPartPlacements _output))
            (if _is_valid
              (Development|PrintString "Yes" true false "(R=0.000000,G=0.660000,B=1.000000,A=1.000000)" 0.0)
              (else
                (Development|PrintString "No" true false "(R=0.000000,G=0.660000,B=1.000000,A=1.000000)" 0.0)))))))))

(fn MakeBuildAssemblyClickable
  (params (Build%20Assembly :type Build%20Assembly%20Pawn%20Object%20Reference))
  (for _array_element (Variables|/Game/Blueprints/BuildAssembly/BuildAssemblyPawn.BuildAssemblyPawn_C|GetBuildParts Build%20Assembly)
    (if (not (Variables|/Game/Blueprints/BuildParts/BuildPart.BuildPart_C|GetIsBaseBuildPart _array_element))
      (AddComponent|AddClickableBuildPartComponent _array_element true))))

(fn CheckValidBuildPartPlacements
  (params (Build%20Part :type Build%20Part%20Object%20Reference))
  (if (BuildParts|BuildPartPlacementValid Build%20Part)
    (for _array_element (Default|GetDescendantBuildParts Build%20Part)
      (if (not (BuildParts|BuildPartPlacementValid _array_element))
        (return false)))
    (return true)
    (else
      (return false))))

(fn MoveChildBuildParts
  (params (ParentBuildPart :type Build%20Part%20Object%20Reference))
  (for _array_element (Default|GetDescendantBuildParts ParentBuildPart)
    (LocalVariables|SetChildBuildPart _array_element)
    (Default|SetBuildPartLocation (BuildAssembly|GetBuildAssemblyPawn) (LocalVariables|GetChildBuildPart) (Default|GetMainConnectionSlot (LocalVariables|GetChildBuildPart)) (Default|GetConnectedSlot (Default|GetMainConnectionSlot (LocalVariables|GetChildBuildPart))))))

(fn RevertBuildPartInstanceData
  (bind _previousbuildpartinstancedatas (Variables|Data|GetPreviousBuildPartInstanceDatas))
  (bind _keys (Utilities|Map|Keys _previousbuildpartinstancedatas))
  (for _array_element _keys
    (Default|RevertInstanceData _array_element (.Value (Utilities|Map|Find _previousbuildpartinstancedatas _array_element)))))

(fn DestroySelectedBuildParts
  (for _array_element (BuildParts|GetSelectedBuildParts)
    (Utilities|IsValid _array_element
      (:Is%20Valid
        (Default|DestroyBuildPart _array_element)))))

(fn GetSelectedBuildParts
  (return (Variables|BuildParts|GetSelectedBuildParts)))

(fn AnyBuildPartsSelected
  (return (> (Utilities|Array|Length (BuildParts|GetSelectedBuildParts)) 0)))

(fn BuildPartPlacementValid
  (params (Build%20Part :type Build%20Part%20Object%20Reference) (ActorsToIgnore :type Array%20of%20Actor%20Object%20References))
  (bind _staticmesh (Variables|/Game/Blueprints/BuildParts/BuildPart.BuildPart_C|GetStaticMesh Build%20Part))
  (Utilities|IsValid Build%20Part
    (:Is%20Valid
      (bind _output_get (LocalVariables|SetAllActorsToIgnore ActorsToIgnore))
      (Utilities|Array|Add _output_get Build%20Part)
      (bind _returnvalue (Collision|ComponentOverlapActors _staticmesh (Transformation|GetWorldTransform _staticmesh) (Utilities|Array|MakeArray "ObjectTypeQuery8") "/Game/Blueprints/BuildParts/BuildPart.BuildPart_C" (LocalVariables|GetAllActorsToIgnore)))
      (if (not _returnvalue)
        (Default|SetBuildPartMaterial Build%20Part (Default|GetDefaultMaterial Build%20Part))
        (return true)
        (else
          (Default|SetBuildPartMaterial Build%20Part "/Game/Materials/InvalidMaterials/M_InvalidMaterial_Inst.M_InvalidMaterial_Inst")
          (return false))))
    (:Is%20Not%20Valid
      (Development|PrintString "Hello"))))

(fn DeleteSelectedBuildParts
  (switch Utilities|FlowControl|Switch|SwitchonBuildPlayMode (Modes|GetBuildPlayMode)
    (:NewEnumerator0
      (switch Utilities|FlowControl|Switch|SwitchonBuildPlayMouseMode (Variables|Modes|GetBuildPlayMouseMode)
        (:NewEnumerator0
          _)
        (:NewEnumerator1
          (Modes|SetBuildPlayMouseMode "NewEnumerator0")))
      (for _array_element (BuildParts|GetSelectedBuildParts)
        (BuildParts|DeleteBuildPart _array_element))
      (BuildParts|UnselectAllSelectedBuildParts)
      (Default|CallBuildAssemblyModified (BuildAssembly|GetBuildAssemblyPawn) true))))

(fn PlaceFirstSelectedBuildPart
  (if (CallFunction|AnyBuildPartsSelected)
    (BuildParts|PlaceBuildPart (Utilities|Array|Get(acopy) (BuildParts|GetSelectedBuildParts)))
    (BuildParts|UnselectAllSelectedBuildParts)))

(fn UnselectBuildPart
  (params (BuildPartToUnselect :type Build%20Part%20Object%20Reference))
  (bind _succeeded_ (Default|SetSelected (Actor|GetComponentbyClass BuildPartToUnselect "/Game/Blueprints/BuildParts/ClickableBuildPartComponent.ClickableBuildPartComponent_C") false))
  (if _succeeded_
    (Utilities|Array|RemoveItem (Variables|BuildParts|GetSelectedBuildParts) BuildPartToUnselect)
    (return true)
    (else
      (return false))))

(fn PickUpFirstSelectedBuildPart
  (if (CallFunction|AnyBuildPartsSelected)
    (BuildParts|PickUpBuildPart (Utilities|Array|Get(acopy) (BuildParts|GetSelectedBuildParts)))))

(fn RemoveSelectedBuildPart
  (params (SelectedBuildPartToRemove :type Build%20Part%20Object%20Reference))
  (Utilities|IsValid SelectedBuildPartToRemove
    (:Is%20Valid
      (bind _succeeded_ (Default|SetSelected (Actor|GetComponentbyClass SelectedBuildPartToRemove "/Game/Blueprints/BuildParts/ClickableBuildPartComponent.ClickableBuildPartComponent_C") false))
      (if _succeeded_
        (Utilities|Array|RemoveItem (Variables|BuildParts|GetSelectedBuildParts) SelectedBuildPartToRemove)
        (Utilities|Map|Remove (Variables|Data|GetPreviousBuildPartInstanceDatas) SelectedBuildPartToRemove)
        (for _array_element (Default|GetDescendantBuildParts SelectedBuildPartToRemove)
          (Utilities|Map|Remove (Variables|Data|GetPreviousBuildPartInstanceDatas) _array_element))
        (Default|CallSelectedBuildPartChanged)))))

(fn DeleteBuildPart
  (params (BuildPartToDelete :type Build%20Part%20Object%20Reference))
  (for _array_element (Default|GetChildBuildParts BuildPartToDelete)
    (BuildParts|DeleteBuildPart _array_element))
  (bind _removed_ (Default|RemoveBuildPart (BuildAssembly|GetBuildAssemblyPawn) BuildPartToDelete))
  (if _removed_
    (Default|DestroyBuildPart BuildPartToDelete)))