(event Custom|BuildAssemblyChanged
  (params (NewBuildAssemblyPawn :type Build%20Assembly%20Pawn%20Object%20Reference))
  (Variables|Game|SetBuildAssemblyPawn NewBuildAssemblyPawn))

(event EventBeginPlay
  (EventDispatchers|BindEventtoBuildAssemblyPawnChanged (Game|GetBuildPlayGameMode) (delegate Custom|BuildAssemblyChanged)))

(event EventTick
  (params (DeltaSeconds :type Float%20%28single-precision%29))
  (CallFunction|ApplyCameraRotations DeltaSeconds))

(event Input|ActionEvents|InputActionSpace
  (params (Key :type Key%20Structure :default "None"))
  ;[1 1 1] Input Action Controls
  (:Pressed
    (Utilities|RunActionMappingInput "NewEnumerator0" :!label _label))
  (:Released
    (goto _label Released)))

(event Input|ActionEvents|InputActionW
  (params (Key :type Key%20Structure :default "None"))
  ;[1 1 1] Input Action Controls
  (:Pressed
    (Utilities|RunActionMappingInput "NewEnumerator1" :!label _label))
  (:Released
    (goto _label Released)))

(event Input|ActionEvents|InputActionD
  (params (Key :type Key%20Structure :default "None"))
  ;[1 1 1] Input Action Controls
  (:Pressed
    (Utilities|RunActionMappingInput "NewEnumerator4" :!label _label))
  (:Released
    (goto _label Released)))

(event Input|ActionEvents|InputActionUp
  (params (Key :type Key%20Structure :default "None"))
  ;[1 1 1] Input Action Controls
  (:Pressed
    (Utilities|RunActionMappingInput "NewEnumerator5" :!label _label))
  (:Released
    (goto _label Released)))

(event Input|ActionEvents|InputActionDown
  (params (Key :type Key%20Structure :default "None"))
  ;[1 1 1] Input Action Controls
  (:Pressed
    (Utilities|RunActionMappingInput "NewEnumerator6" :!label _label))
  (:Released
    (goto _label Released)))

(event Input|ActionEvents|InputActionLeft
  (params (Key :type Key%20Structure :default "None"))
  ;[1 1 1] Input Action Controls
  (:Pressed
    (Utilities|RunActionMappingInput "NewEnumerator7" :!label _label))
  (:Released
    (goto _label Released)))

(event Input|ActionEvents|InputActionRight
  (params (Key :type Key%20Structure :default "None"))
  ;[1 1 1] Input Action Controls
  (:Pressed
    (Utilities|RunActionMappingInput "NewEnumerator8" :!label _label))
  (:Released
    (goto _label Released)))

(event Input|ActionEvents|InputActionCtrl
  (params (Key :type Key%20Structure :default "None"))
  ;[1 1 1] Input Action Controls
  (:Pressed
    (Utilities|RunActionMappingInput "NewEnumerator9" :!label _label))
  (:Released
    (goto _label Released)))

(event Input|ActionEvents|InputActionShift
  (params (Key :type Key%20Structure :default "None"))
  ;[1 1 1] Input Action Controls
  (:Pressed
    (Utilities|RunActionMappingInput "NewEnumerator10" :!label _label))
  (:Released
    (goto _label Released)))

(event Input|ActionEvents|InputActionAlt
  (params (Key :type Key%20Structure :default "None"))
  ;[1 1 1] Input Action Controls
  (:Pressed
    (Utilities|RunActionMappingInput "NewEnumerator11" :!label _label))
  (:Released
    (goto _label Released)))

(event Input|ActionEvents|InputActionEnter
  (params (Key :type Key%20Structure :default "None"))
  ;[1 1 1] Input Action Controls
  (:Pressed
    (Utilities|RunActionMappingInput "NewEnumerator12" :!label _label))
  (:Released
    (goto _label Released)))

(event Input|ActionEvents|InputActionToggleMoveMode
  (params (Key :type Key%20Structure :default "None"))
  (bind _buildplaygamemode (Game|GetBuildPlayGameMode))
  (:Pressed
    (switch Utilities|FlowControl|Switch|SwitchonBuildPlayMode (Default|GetBuildPlayMode _buildplaygamemode)
      (:NewEnumerator0
        (switch Utilities|FlowControl|Switch|SwitchonBuildPlayMouseMode (Variables|/Game/Blueprints/BuildPlayMode/BuildPlayGameMode.BuildPlayGameMode_C|GetBuildPlayMouseMode _buildplaygamemode)
          (:NewEnumerator0
            (Default|SetBuildPlayMouseMode _buildplaygamemode "NewEnumerator1"))
          (:NewEnumerator1
            (Default|SetBuildPlayMouseMode _buildplaygamemode "NewEnumerator0")))))))

(event Input|ActionEvents|InputActionRotateBuildPart
  (params (Key :type Key%20Structure :default "None"))
  (bind _buildplaygamemode (Game|GetBuildPlayGameMode))
  (bind _currentbuildpart (Default|GetSelectedBuildPart _buildplaygamemode))
  (:Pressed
    (Utilities|IsValid _currentbuildpart
      (:Is%20Valid
        (Default|IncrementRotation90 _currentbuildpart)))))

(event Input|ActionEvents|InputActionRevertOperation
  (params (Key :type Key%20Structure :default "None"))
  (:Pressed
    (Default|RevertOperation (Game|GetBuildPlayGameMode))))

(event Input|ActionEvents|InputActionDelete
  (params (Key :type Key%20Structure :default "None"))
  (:Pressed
    (Default|DeleteSelectedBuildPart (Game|GetBuildPlayGameMode))))

(event Input|ActionEvents|InputActionIncrementConnectionSlotSeed
  (params (Key :type Key%20Structure :default "None"))
  (:Pressed
    (Default|IncrementConnectionSlotSeed (Default|GetBuildPlayGameState (Game|GetBuildPlayGameMode)))))

(event Input|ActionEvents|InputActionA
  (params (Key :type Key%20Structure :default "None"))
  ;[1 1 1] Input Action Controls
  (:Pressed
    (Utilities|RunActionMappingInput "NewEnumerator2" :!label _label))
  (:Released
    (goto _label Released)))

(event Input|ActionEvents|InputActionCameraZoomIn
  (params (Key :type Key%20Structure :default "None"))
  ;[1 1 1] Move Camera
  (:Pressed
    (CallFunction|ZoomCamera 0.9)))

(event Input|ActionEvents|InputActionCameraZoomOut
  (params (Key :type Key%20Structure :default "None"))
  ;[1 1 1] Move Camera
  (:Pressed
    (CallFunction|ZoomCamera 1.1111)))

(event Input|ActionEvents|InputActionS
  (params (Key :type Key%20Structure :default "None"))
  ;[1 1 1] Input Action Controls
  (:Pressed
    (Utilities|RunActionMappingInput "NewEnumerator3" :!label _label))
  (:Released
    (goto _label Released)))

(event Input|AxisEvents|InputAxisRotateCameraUp
  (params (AxisValue :type Float%20%28single-precision%29))
  ;[1 1 1] Move Camera
  (CallFunction|AddRotation 0.0 AxisValue))

(event Input|AxisEvents|InputAxisRotateCameraDown
  (params (AxisValue :type Float%20%28single-precision%29))
  ;[1 1 1] Move Camera
  (CallFunction|AddRotation 0.0 AxisValue))

(event Input|AxisEvents|InputAxisRotateCameraLeft
  (params (AxisValue :type Float%20%28single-precision%29))
  ;[1 1 1] Move Camera
  (CallFunction|AddRotation AxisValue 0.0))

(event Input|AxisEvents|InputAxisRotateCameraRight
  (params (AxisValue :type Float%20%28single-precision%29))
  ;[1 1 1] Move Camera
  (CallFunction|AddRotation AxisValue 0.0))

(fn ConstructionScript)

(fn GetBuildPlayGameMode
  (Utilities|IsValid (Variables|Game|GetBuildPlayGameMode)
    (:Is%20Valid
      _)
    (:Is%20Not%20Valid
      (bind _asbuild_play_game_mode (Utilities|Casting|CastToBuildPlayGameMode (Game|GetGameMode))
        (:then
          (Variables|Game|SetBuildPlayGameMode _asbuild_play_game_mode))
        (:CastFailed
          _))))
  (return (Variables|Game|GetBuildPlayGameMode)))

(fn GetWorldLocationUnderMouseCursor
  (params (ActorsToIgnore :type Array%20of%20Actor%20Object%20References))
  (bind (_locationx _locationy) (Game|Player|GetMousePosition))
  (bind _returnvalue (Game|GetPlayerController 0))
  (bind (_worldposition _worlddirection _returnvalue_2) (Class|GameplayStatics|DeprojectScreentoWorld _returnvalue (Math|Vector2D|MakeVector2D _locationx _locationy)))
  (if _returnvalue_2
    (bind (_outhit _returnvalue_3) (Collision|LineTraceByChannel _worldposition (+ _worldposition (* _worlddirection 5e+03)) "TraceTypeQuery1" false ActorsToIgnore "None"))
    (return (.Location (Collision|BreakHitResult _outhit)) _returnvalue_3)
    (else
      (return "0, 0, 0" false))))

(fn RotateCamera
  (params (Y%20%28Pitch%29 :type Float%20%28single-precision%29) (Z%20%28Yaw%29 :type Float%20%28single-precision%29))
  (Default|AddCameraLocalRotation (Game|GetBuildAssemblyPawn) Y%20%28Pitch%29 Z%20%28Yaw%29))

(fn ZoomCamera
  (params (Zoom%20Multiplier :type Float%20%28double-precision%29))
  (Default|SetCameraZoom (Game|GetBuildAssemblyPawn) Zoom%20Multiplier))

(fn GetBuildPartUnderMouseCursor
  (params (ActorsToIgnore :type Array%20of%20Actor%20Object%20References))
  (bind (_locationx _locationy) (Game|Player|GetMousePosition))
  (bind _returnvalue (Game|GetPlayerController 0))
  (bind (_worldposition _worlddirection _returnvalue_2) (Class|GameplayStatics|DeprojectScreentoWorld _returnvalue (Math|Vector2D|MakeVector2D _locationx _locationy)))
  (if _returnvalue_2
    (bind _outhit (Collision|LineTraceByChannel _worldposition (+ _worldposition (* _worlddirection 5e+03)) "TraceTypeQuery1" false ActorsToIgnore "None"))
    (bind _asbuild_part (Utilities|Casting|CastToBuildPart (.HitActor (Collision|BreakHitResult _outhit)))
      (:then
        (return _asbuild_part true))
      (:CastFailed
        (return 0 false)))
    (else
      (return 0 false))))

(fn ApplyCameraRotations
  (params (Delta%20Seconds :type Float%20%28double-precision%29))
  (bind _returnvalue (Math|Float|MakeLiteralFloat 1e+02))
  (CallFunction|RotateCamera (* (Variables|Default|GetCameraPitchRotation) Delta%20Seconds _returnvalue) (* (Variables|Default|GetCameraYawRotation) Delta%20Seconds _returnvalue))
  (Variables|Default|SetCameraYawRotation 0.0)
  (Variables|Default|SetCameraPitchRotation 0.0))

(fn AddRotation
  (params (Delta%20Yaw :type Float%20%28double-precision%29) (Delta%20Pitch :type Float%20%28double-precision%29))
  (Variables|Default|SetCameraYawRotation (+ (Variables|Default|GetCameraYawRotation) Delta%20Yaw))
  (Variables|Default|SetCameraPitchRotation (+ (Variables|Default|GetCameraPitchRotation) Delta%20Pitch)))

(fn GetBuildAssemblyPawn
  (Utilities|IsValid (Variables|Game|GetBuildAssemblyPawn)
    (:Is%20Valid
      _)
    (:Is%20Not%20Valid
      (bind _asbuild_assembly_pawn (Utilities|Casting|CastToBuildAssemblyPawn (Game|Player|GetPlayerPawn 0))
        (:then
          (Variables|Game|SetBuildAssemblyPawn _asbuild_assembly_pawn))
        (:CastFailed
          _))))
  (return (Variables|Game|GetBuildAssemblyPawn)))