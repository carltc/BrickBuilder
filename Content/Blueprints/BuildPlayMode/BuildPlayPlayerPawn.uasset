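; Player pawn for build/play mode that carries a build assembly and provides an orbit camera on a spring arm.
; AddBuildAssembly detaches any previous assembly, moves the pawn to the new one and attaches it, keeping world transforms.
; Camera functions apply pitch locally and yaw in world space to avoid roll, and zoom by scaling arm length within a clamped range.
; Event graph is empty, so other classes drive it through these functions.
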(event EventBeginPlay)

(event Collision|EventActorBeginOverlap
  (params (OtherActor :type Actor%20Object%20Reference)))

(event EventTick
  (params (DeltaSeconds :type Float%20%28single-precision%29)))

(fn ConstructionScript)

(fn AddBuildAssembly
  (params (NewBuildAssembly :type Build%20Assembly%20Object%20Reference))
  (Utilities|IsValid (Variables|Default|GetBuildAssembly)
    (:Is%20Valid
      (Transformation|DetachFromActor (Variables|Default|GetBuildAssembly) "KeepWorld" "KeepWorld" "KeepWorld"))
    (:Is%20Not%20Valid
      _))
  (Transformation|SetActorLocation (Default|GetWorldLocation NewBuildAssembly) false false)
  (bind _output_get (Variables|Default|SetBuildAssembly NewBuildAssembly))
  (Transformation|AttachActorToActor _output_get self "None" "KeepWorld" "KeepWorld" "KeepWorld" true))

(fn GetBuildAssembly
  (return (Variables|Default|GetBuildAssembly)))

(fn AddCameraLocalRotation
  (params (Y%20%28Pitch%29 :type Float%20%28single-precision%29) (Z%20%28Yaw%29 :type Float%20%28single-precision%29))
  (bind _springarm (Variables|Default|GetSpringArm))
  (Transformation|AddLocalRotation _springarm (Math|Rotator|MakeRotator 0.0 Y%20%28Pitch%29 0.0) false false)
  (Transformation|AddWorldRotation _springarm (Math|Rotator|MakeRotator 0.0 0.0 Z%20%28Yaw%29) false false))

(fn SetCameraZoom
  (params (Zoom%20Multiplier :type Float%20%28double-precision%29))
  (bind _springarm (Variables|Default|GetSpringArm))
  (Variables|/Script/Engine.SpringArmComponent|SetTargetArmLength _springarm (Math|Float|Clamp(Float) (* Zoom%20Multiplier (Variables|/Script/Engine.SpringArmComponent|GetTargetArmLength _springarm)) 0.0 1e+03)))