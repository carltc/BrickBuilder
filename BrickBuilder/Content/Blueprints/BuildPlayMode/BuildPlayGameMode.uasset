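; Game mode for the build/play mode, where the player builds assemblies from parts.
; On BeginPlay it shows the mouse cursor with game-and-UI input, then spawns a BuildAssembly at the origin and registers it with the player pawn.
; It also offers SpawnBuildPart to spawn a given part class at a location, owned by the player controller.
; The BuildPlayPlayerPawn reference is lazily cast from player pawn 0 and cached.
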(event EventBeginPlay
  (Utilities|FlowControl|Sequence
    (:then_0
      (Input|SetInputModeGameandUI (Game|GetPlayerController 0) 0 "DoNotLock" false false)
      (Class|GameplayStatics|SetViewportMouseCaptureMode "NoCapture")
      (Variables|/Script/Engine.PlayerController|SetbShowMouseCursor (Game|GetPlayerController 0) true))
    (:then_1
      (CallFunction|SpawnBuildAssembly))))

(event EventTick
  (params (DeltaSeconds :type Float%20%28single-precision%29)))

(fn ConstructionScript)

(fn SpawnBuildPart
  (params (Build%20Part%20Class :type Build%20Part%20Class%20Reference) (Location :type Vector))
  (bind _returnvalue (Game|SpawnActorfromClass Build%20Part%20Class (Math|Transform|MakeTransform Location) "Undefined" "MultiplyWithRoot" (Game|GetPlayerController 0) 0))
  (return _returnvalue))

(fn SpawnBuildAssembly
  (bind _returnvalue (Game|SpawnActorfromClass "/Game/Blueprints/BuildAssembly/BuildAssembly.BuildAssembly_C" (Math|Transform|MakeTransform "0, 0, 0") "Undefined" "MultiplyWithRoot" 0 0))
  (Default|AddBuildAssembly (CallFunction|GetBuildPlayPlayerPawn) _returnvalue))

(fn GetBuildPlayPlayerPawn
  (Utilities|IsValid (Variables|Default|GetBuildPlayPlayerPawn)
    (:Is%20Valid
      _)
    (:Is%20Not%20Valid
      (bind _asbuild_play_player_pawn (Utilities|Casting|CastToBuildPlayPlayerPawn (Game|Player|GetPlayerPawn 0))
        (:then
          (Variables|Default|SetBuildPlayPlayerPawn _asbuild_play_player_pawn))
        (:CastFailed
          _))))
  (return (Variables|Default|GetBuildPlayPlayerPawn)))